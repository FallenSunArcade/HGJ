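; Ferris wheel actor for the Carnival map that spins its wheel mesh continuously.
; Tick adds relative roll to the wheel, scaled by RotationSpeed and delta time for frame-rate-independent motion.
; BeginPlay sets all 36 cabins upright in world space, matching the wheel's yaw; Tick does not re-level them.
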(event EventBeginPlay
  (Transformation|SetWorldRotation (Variables|Default|GetCabin7) (Math|Rotator|MakeRotator 0.0 0.0 (.yaw (Transformation|GetWorldRotation (Variables|Default|GetWheelMesh)))) false false))

(event EventTick
  (params (DeltaSeconds :type Float%20%28single-precision%29))
  (Transformation|AddRelativeRotation (Variables|Default|GetWheelMesh) (Math|Rotator|MakeRotator (* DeltaSeconds (Variables|Default|GetRotationSpeed)) 0.0 0.0) false false))

(fn ConstructionScript)