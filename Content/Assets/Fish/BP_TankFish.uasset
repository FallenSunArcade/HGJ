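; BP_TankFish is a randomly sized fish character that wanders by timed launches in random directions, with timelines easing its rotation.
; BeginPlay sets all its face and tail morph targets to full.
; Damage lowers Health, and death disables collision and floats the body upward.
; An evil transformation that morphs, rescales and starts chasing the player remains in disconnected nodes, so the overlap and Spawner events do not trigger it.
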(event OnComponentBeginOverlap(CollisionCapsule)
  (params (OverlappedComponent :type Primitive%20Component%20Object%20Reference) (OtherActor :type Actor%20Object%20Reference) (OtherComp :type Primitive%20Component%20Object%20Reference) (OtherBodyIndex :type Integer) (bFromSweep :type Boolean) (SweepResult :type Hit%20Result%20Structure%20%28by%20ref%29)))

(event OnComponentEndOverlap(CollisionCapsule)
  (params (OverlappedComponent :type Primitive%20Component%20Object%20Reference) (OtherActor :type Actor%20Object%20Reference) (OtherComp :type Primitive%20Component%20Object%20Reference) (OtherBodyIndex :type Integer)))

(event OnComponentBeginOverlap(AttackHitCollision)
  (params (OverlappedComponent :type Primitive%20Component%20Object%20Reference) (OtherActor :type Actor%20Object%20Reference) (OtherComp :type Primitive%20Component%20Object%20Reference) (OtherBodyIndex :type Integer) (bFromSweep :type Boolean) (SweepResult :type Hit%20Result%20Structure%20%28by%20ref%29))
  ;[1 1 1] PlayerHitable
  (if (== (Utilities|Array|Get(acopy) (Variables|/Script/Engine.Actor|GetTags OtherActor)) "Player")
    (Variables|Default|SetPlayerInAttackCollision true)))

(event OnComponentEndOverlap(AttackHitCollision)
  (params (OverlappedComponent :type Primitive%20Component%20Object%20Reference) (OtherActor :type Actor%20Object%20Reference) (OtherComp :type Primitive%20Component%20Object%20Reference) (OtherBodyIndex :type Integer))
  ;[1 1 1] PlayerHitable
  (if (== (Utilities|Array|Get(acopy) (Variables|/Script/Engine.Actor|GetTags OtherActor)) "Player")
    (Variables|Default|SetPlayerInAttackCollision false)))

(event Custom|FollowPlayer
  ;[1 1 1] FollowPlayer
  (Character|LaunchCharacter (* (Math|Vector|Normalize (- (Transformation|GetActorLocation (Variables|Default|GetPlayer)) (Transformation|GetActorLocation))) (Variables|Default|GetSpeedNormal)) true true))

(event Custom|HitEnemy
  ;[1 1 1] PlayerHitable
  (Game|Damage|ApplyDamage (stale OnComponentBeginOverlap(AttackHitCollision) OtherActor) 5.0 0 0))

(event Custom|RandomMovement
  (bind _returnvalue (Transformation|GetActorLocation))
  ;[1 1 1] RandomMovement
  (if (not (Variables|Default|GetEvilSpawned))
    (if (not (Variables|Default|GetDead))
      (Variables|Default|SetLookRotation (Math|Vector|MakeVector (Math|Random|RandomFloatinRange -1.0 1.0) (Math|Random|RandomFloatinRange -1.0 1.0) (Math|Random|RandomFloatinRange -1.0 1.0)))
      (Character|LaunchCharacter (* (Variables|Default|GetLookRotation) (Variables|Default|GetSpeedNormal)) false false)
      ;[1 1 1] RotateFish
      (bind _newtrack_0 (Timeline|Timeline_4 PlayFromStart)
        (:Update
          (Transformation|SetActorRotation (Math|Interpolation|RInterpTo (Transformation|GetActorRotation) (Math|Rotator|FindLookatRotation _returnvalue (+ _returnvalue (Variables|Default|GetLookRotation))) _newtrack_0 0.5)))))))

(event Custom|Spawner)

(event Custom|LootAtMother
  (bind _returnvalue (Transformation|GetActorLocation))
  (bind _returnvalue_2 (Transformation|GetActorLocation))
  ;[1 1 1] RotateFish
  (bind _newtrack_0 (Timeline|Timeline_6 PlayFromStart)
    (:Update
      (Transformation|SetActorRotation (Math|Interpolation|RInterpTo (Transformation|GetActorRotation) (Math|Rotator|FindLookatRotation _returnvalue (+ _returnvalue (Variables|Default|GetLookRotation))) _newtrack_0 0.5))
      ;[1 1 1] RotateFish
      (bind _newtrack_0_2 (Timeline|Timeline_4 Stop)
        (:Update
          (Transformation|SetActorRotation (Math|Interpolation|RInterpTo (Transformation|GetActorRotation) (Math|Rotator|FindLookatRotation _returnvalue_2 (+ _returnvalue_2 (Variables|Default|GetLookRotation))) _newtrack_0_2 0.5)))))))

(event EventBeginPlay
  (bind _returnvalue (Math|Random|RandomFloatinRange 0.1 0.5))
  (Transformation|SetWorldScale3D (Variables|Collision|GetCapsuleComponent) (Math|Vector|MakeVector _returnvalue _returnvalue _returnvalue))
  (Utilities|Time|SetTimerbyFunctionName 0 "RandomMovement" (Math|Random|RandomFloatinRange 2.0 5.0) true)
  (Components|SkeletalMesh|SetMorphTarget (Variables|Character|GetMesh) "eyes" 1.0 true)
  (bind _asbp_player (Utilities|Casting|CastToBP_Player (Game|GetPlayerCharacter 0)))
  (Variables|Default|SetPlayer _asbp_player)
  (Variables|Default|SetNewVar (Math|Random|RandomFloatinRange 0.5 2.0))
  (Variables|Default|SetNewVar_0 (Math|Random|RandomFloatinRange 0.5 2.0))
  (Variables|Default|SetNewVar_1 (Math|Random|RandomFloatinRange 0.5 2.0))
  (Components|SkeletalMesh|SetMorphTarget (Variables|Character|GetMesh) "eyes2" 1.0 true)
  (Components|SkeletalMesh|SetMorphTarget (Variables|Character|GetMesh) "tail" 1.0 true)
  (Components|SkeletalMesh|SetMorphTarget (Variables|Character|GetMesh) "mouth" 1.0 true)
  (Components|SkeletalMesh|SetMorphTarget (Variables|Character|GetMesh) "mouth2" 1.0 true)
  (Components|SkeletalMesh|SetMorphTarget (Variables|Character|GetMesh) "teeth" 1.0 true))

(event Game|Damage|EventAnyDamage
  (params (Damage :type Float%20%28single-precision%29) (DamageType :type Damage%20Type%20Object%20Reference) (InstigatedBy :type Controller%20Object%20Reference) (DamageCauser :type Actor%20Object%20Reference))
  (bind _returnvalue (Transformation|GetActorRotation))
  ;[1 1 1] Damage+ Death
  (bind _output_get (Variables|Default|SetHealth (- (Variables|Default|GetHealth) Damage)))
  (if (< _output_get 0.0)
    (Variables|Default|SetDead true)
    (Pawn|Components|CharacterMovement|SetMovementMode (Variables|Character|GetCharacterMovement) "MOVE_None" 0)
    (Collision|SetCollisionEnabled (Variables|Collision|GetCapsuleComponent) "NoCollision")
    (Timeline|Timeline_5 Play
      (:Update
        (Transformation|SetActorRotation (Math|Interpolation|RInterpTo (Math|Rotator|MakeRotator (.roll _returnvalue) (.pitch _returnvalue) (.yaw _returnvalue)) (Math|Rotator|MakeRotator 0.0 0.0 (.yaw _returnvalue)) (Utilities|Time|GetWorldDeltaSeconds) 1.0))))
    (else
      (CallFunction|Spawner))))

(event EventTick
  (params (DeltaSeconds :type Float%20%28single-precision%29))
  (bind _returnvalue (Transformation|GetActorLocation))
  (bind _player (Variables|Default|GetPlayer))
  (bind _returnvalue_2 (Transformation|GetActorLocation _player))
  (bind _returnvalue_3 (Math|Rotator|FindLookatRotation _returnvalue _returnvalue_2))
  ;[1 1 1] EventTick
  (if (Variables|Default|GetDead)
    (Transformation|SetActorLocation (+ (Transformation|GetActorLocation) "0.000000,0.000000,5.000000") false false)
    (elif (Variables|Default|GetEvilSpawned)
      (Transformation|SetActorRotation (Math|Interpolation|RInterpTo (Transformation|GetActorRotation) (Math|Rotator|MakeRotator (.roll _returnvalue_3) (.pitch _returnvalue_3) (.yaw _returnvalue_3)) (Utilities|Time|GetWorldDeltaSeconds) 3.0)))))

(fn ConstructionScript)