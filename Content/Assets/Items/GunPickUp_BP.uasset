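; GunPickUp_BP is a pickup actor that gives the player a gun.
; When its sphere is overlapped by an actor whose first tag is "Player", it casts player character 0 to BP_Player and calls ActivateGun.
; It then prints a debug message, destroys itself and plays a 2D pickup sound event.
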(event OnComponentBeginOverlap(Sphere)
  (params (OverlappedComponent :type Primitive%20Component%20Object%20Reference) (OtherActor :type Actor%20Object%20Reference) (OtherComp :type Primitive%20Component%20Object%20Reference) (OtherBodyIndex :type Integer) (bFromSweep :type Boolean) (SweepResult :type Hit%20Result%20Structure%20%28by%20ref%29))
  (bind _tags (Variables|/Script/Engine.Actor|GetTags OtherActor))
  (if (Utilities|Array|IsValidIndex _tags)
    (if (== (Utilities|Array|Get(acopy) _tags) "Player")
      (bind _asbp_player (Utilities|Casting|CastToBP_Player (Game|GetPlayerCharacter 0)))
      (Default|ActivateGun _asbp_player)
      (Development|PrintString "Gun Activated")
      (Actor|DestroyActor)
      (Class|FMODBlueprintStatics|PlayEvent2D "/Game/FMOD/Events/Items/Pickup_Gun.Pickup_Gun"))))

(event EventBeginPlay)

(event Collision|EventActorBeginOverlap
  (params (OtherActor :type Actor%20Object%20Reference)))

(event EventTick
  (params (DeltaSeconds :type Float%20%28single-precision%29)))

(fn ConstructionScript)