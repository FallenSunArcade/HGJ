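; Golden gun pickup item that upgrades the player's weapon when touched.
; A sphere overlap checks whether the other actor's first tag is "Player", then casts the player character to BP_Player.
; It overrides that gun's damage, magazine size and fire pause, swaps the gun mesh material to gold, then destroys itself.
; A disconnected ActivateGun call with a debug print remains unused.
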(event OnComponentBeginOverlap(Sphere)
  (params (OverlappedComponent :type Primitive%20Component%20Object%20Reference) (OtherActor :type Actor%20Object%20Reference) (OtherComp :type Primitive%20Component%20Object%20Reference) (OtherBodyIndex :type Integer) (bFromSweep :type Boolean) (SweepResult :type Hit%20Result%20Structure%20%28by%20ref%29))
  (bind _tags (Variables|/Script/Engine.Actor|GetTags OtherActor))
  (if (Utilities|Array|IsValidIndex _tags)
    (if (== (Utilities|Array|Get(acopy) _tags) "Player")
      (bind _asbp_player (Utilities|Casting|CastToBP_Player (Game|GetPlayerCharacter 0)))
      (Variables|/Game/BP_Player.BP_Player_C|SetDamageGun _asbp_player 25.0)
      (Rendering|Material|SetMaterial (Variables|/Game/BP_Player.BP_Player_C|GetMesh_Gun _asbp_player) 0 "/Game/Assets/Items/Gun/M_GoldenGun_2.M_GoldenGun_2")
      (Variables|/Game/BP_Player.BP_Player_C|SetMagazineSize _asbp_player 2e+01)
      (Variables|/Game/BP_Player.BP_Player_C|SetPauseBetweenShots _asbp_player 0.25)
      (Actor|DestroyActor))))

(event EventBeginPlay)

(event Collision|EventActorBeginOverlap
  (params (OtherActor :type Actor%20Object%20Reference)))

(event EventTick
  (params (DeltaSeconds :type Float%20%28single-precision%29)))

(fn ConstructionScript)