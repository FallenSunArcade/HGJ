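; Small Ferris wheel actor that spins its wheel mesh, cycles light color and plays FMOD carnival audio.
; Tick rolls the wheel while Rotating is set and advances the Hue parameter on a dynamic light material created at construction.
; BeginPlay levels the cabins and either adds an audio component in menus or plays positioned music with Dark_Layer zeroed.
; StopWheel halts rotation and wheel audio, then plays a stopping sound.
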(event Custom|StopWheel
  (Variables|Default|SetRotating? false)
  (Audio|Components|Audio|Stop (Variables|Default|GetFerris_Wheel_Audio))
  (Class|FMODBlueprintStatics|PlayEvent2D "/Game/FMOD/Events/Buildings/Ferris_Wheel_Stopping.Ferris_Wheel_Stopping"))

(event Custom|BeginPlay1
  (if (Variables|Default|GetInMenu?)
    (AddComponent|AddFMODAudioComponent false)
    (else
      (bind _returnvalue (Class|FMODBlueprintStatics|PlayEventatLocation "/Game/FMOD/Events/Music/Music_carnival.Music_carnival" (Math|Conversions|ToTransform(Vector) (Transformation|GetActorLocation))))
      (Class|FMODBlueprintStatics|EventInstancePlay _returnvalue)
      (bind _returnvalue_2 (Class|FMODBlueprintStatics|EventInstanceIsValid _returnvalue))
      (if _returnvalue_2
        (Class|FMODBlueprintStatics|EventInstanceSetParameter _returnvalue "Dark_Layer" 0.0)))))

(event EventBeginPlay
  (CallFunction|BeginPlay1)
  (Transformation|SetWorldRotation (Variables|Default|GetCabin7) (Math|Rotator|MakeRotator 0.0 0.0 (.yaw (Transformation|GetWorldRotation (Variables|Default|GetWheelMesh)))) false false))

(event EventTick
  (params (DeltaSeconds :type Float%20%28single-precision%29))
  (CallFunction|RotateFerrisWheel DeltaSeconds)
  (CallFunction|ChangeLightColor DeltaSeconds))

(fn ConstructionScript
  (bind _returnvalue (Rendering|Material|CreateDynamicMaterialInstance (Variables|Default|GetWheelMesh) 1 "/Game/Assets/FerrisWheel/Materials/MI_FerrisWheel_Lights.MI_FerrisWheel_Lights" "None" :!class /Script/Engine.PrimitiveComponent))
  (bind _output_get (Variables|Default|SetLightMaterialInstance _returnvalue))
  (Rendering|Material|SetScalarParameterValue _output_get "Hue" (Variables|Default|GetLightBrightness) :!class /Script/Engine.MaterialInstanceDynamic))

(fn RotateFerrisWheel
  (params (DeltaSeconds :type Float%20%28double-precision%29))
  (if (Variables|Default|GetRotating?)
    (Transformation|AddRelativeRotation (Variables|Default|GetWheelMesh) (Math|Rotator|MakeRotator (* DeltaSeconds (Variables|Default|GetRotationSpeed)) 0.0 0.0) false false)))

(fn ChangeLightColor
  (params (DeltaSeconds :type Float%20%28double-precision%29))
  (bind _lightmaterialinstance (Variables|Default|GetLightMaterialInstance))
  (bind _returnvalue (Rendering|Material|GetScalarParameterValue _lightmaterialinstance "Hue" :!class /Script/Engine.MaterialInstanceDynamic))
  (Rendering|Material|SetScalarParameterValue _lightmaterialinstance "Hue" (+ _returnvalue (* DeltaSeconds (Variables|Default|GetLightColorChangeSpeed))) :!class /Script/Engine.MaterialInstanceDynamic))