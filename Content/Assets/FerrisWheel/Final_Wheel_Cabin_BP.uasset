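; Ferris wheel cabin that acts as the game's ending trigger, lifting itself when the player enters its box.
; Overlap by an actor whose first tag is Player disables player movement and starts a Timeline.
; Each update interpolates the cabin upward, using the track as FInterpTo's delta time, and fires the Ferris_Wheel FMOD event again.
; On finish, it sets the GameInstance state to GameEnd and opens Lvl1_Carnival.
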(event OnComponentBeginOverlap(Box)
  (params (OverlappedComponent :type Primitive%20Component%20Object%20Reference) (OtherActor :type Actor%20Object%20Reference) (OtherComp :type Primitive%20Component%20Object%20Reference) (OtherBodyIndex :type Integer) (bFromSweep :type Boolean) (SweepResult :type Hit%20Result%20Structure%20%28by%20ref%29))
  (bind _returnvalue (Transformation|GetActorLocation))
  (if (== (Utilities|Array|Get(acopy) (Variables|/Script/Engine.Actor|GetTags OtherActor)) "Player")
    (bind _asbp_player (Utilities|Casting|CastToBP_Player (Game|GetPlayerCharacter 0)))
    (Variables|/Game/BP_Player.BP_Player_C|SetMovementDisabled _asbp_player true)
    (bind _newtrack_0 (Timeline|Timeline Play)
      (:Update
        (Transformation|SetActorLocation (Math|Vector|MakeVector (.x _returnvalue) (.y _returnvalue) (Math|Interpolation|FInterpTo (.z _returnvalue) (+ (.z _returnvalue) 1e+03) _newtrack_0 1.0)) false false)
        (Class|FMODBlueprintStatics|PlayEvent2D "/Game/FMOD/Events/Buildings/Ferris_Wheel.Ferris_Wheel"))
      (:Finished
        (bind _asbp_game_instance (Utilities|Casting|CastToBP_GameInstance (Game|GetGameInstance)))
        (Class|HGGameInstance|SetGameState _asbp_game_instance "GameEnd")
        (Game|OpenLevel(byObjectReference) "/Game/Maps/Lvl1_Carnival.Lvl1_Carnival")))))

(event EventBeginPlay)

(event Collision|EventActorBeginOverlap
  (params (OtherActor :type Actor%20Object%20Reference)))

(event EventTick
  (params (DeltaSeconds :type Float%20%28single-precision%29)))

(fn ConstructionScript)