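; Whack-a-mole target that randomly pops up and ducks down once the game has started, sometimes appearing as an ex-wife head with a bloody material instead of a mole.
; Looping GetUp and GetDown timers roll a small chance to switch state, then timelines interpolate the mesh between up and down locations.
; A collision sphere tracks hammer overlap through component tags; damage only plays a punch sound, and HitMole is empty.
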(event OnComponentBeginOverlap(CollisionSphere)
  (params (OverlappedComponent :type Primitive%20Component%20Object%20Reference) (OtherActor :type Actor%20Object%20Reference) (OtherComp :type Primitive%20Component%20Object%20Reference) (OtherBodyIndex :type Integer) (bFromSweep :type Boolean) (SweepResult :type Hit%20Result%20Structure%20%28by%20ref%29))
  (bind _componenttags (Variables|/Script/Engine.ActorComponent|GetComponentTags OtherComp))
  (if (Utilities|Array|IsValidIndex _componenttags)
    (if (== (Utilities|Array|Get(acopy) _componenttags) "Hammer")
      (Variables|Default|SetHammeroverTarget true))))

(event OnComponentEndOverlap(CollisionSphere)
  (params (OverlappedComponent :type Primitive%20Component%20Object%20Reference) (OtherActor :type Actor%20Object%20Reference) (OtherComp :type Primitive%20Component%20Object%20Reference) (OtherBodyIndex :type Integer))
  (bind _componenttags (Variables|/Script/Engine.ActorComponent|GetComponentTags OverlappedComponent))
  (if (Utilities|Array|IsValidIndex _componenttags)
    (if (== (Utilities|Array|Get(acopy) _componenttags) "Hammer")
      (Variables|Default|SetHammeroverTarget false))))

(event Custom|HitMole)

(event Custom|GetDown
  (bind _minimole (Variables|Default|GetMiniMole))
  (if (Variables|Default|GetGameHasStarted)
    (if (not (Variables|Default|GetDown))
      (if (> (Math|Random|RandomFloatinRange 0.0 1.0) 0.98)
        (Variables|Default|SetDown true)
        (AddComponent|AddFMODAudioComponent false)
        (bind _newtrack_0 (Timeline|Timeline_1 PlayFromStart)
          (:Update
            (Transformation|SetRelativeLocation _minimole (Math|Interpolation|VInterpTo (Variables|/Script/Engine.SceneComponent|GetRelativeLocation _minimole) (Variables|/Script/Engine.SceneComponent|GetRelativeLocation (Variables|Default|GetDownLocation)) _newtrack_0 1.0) false false)))))))

(event Custom|GetUp
  (bind _minimole (Variables|Default|GetMiniMole))
  (if (Variables|Default|GetGameHasStarted)
    (if (Variables|Default|GetDown)
      (if (> (Math|Random|RandomFloatinRange 0.0 1.0) 0.98)
        (if (< (Math|Random|RandomFloatinRange 0.0 1.0) 0.3)
          (Components|StaticMesh|SetStaticMesh (Variables|Default|GetMiniMole) "/Game/Assets/HumanHeads/exwifehead.exwifehead")
          (Variables|Default|SetbIsHead true)
          (Rendering|Material|SetMaterial _minimole 0 (Variables|Default|GetBloodyMaterial))
          (else
            (Components|StaticMesh|SetStaticMesh (Variables|Default|GetMiniMole) "/Game/Assets/Enemies/Mole/MiniMole.MiniMole")
            (Variables|Default|SetbIsHead false)
            (Rendering|Material|SetMaterial _minimole 0 "/Game/Assets/Enemies/Mole/Textures/MiniMole_Mat.MiniMole_Mat")))
        (Variables|Default|SetDown false)
        (AddComponent|AddFMODAudioComponent false)
        (bind _newtrack_0 (Timeline|Timeline_0 PlayFromStart)
          (:Update
            (Transformation|SetRelativeLocation (Variables|Default|GetMiniMole) (Math|Interpolation|VInterpTo (Variables|/Script/Engine.SceneComponent|GetRelativeLocation (Variables|Default|GetMiniMole)) (Variables|/Script/Engine.SceneComponent|GetRelativeLocation (Variables|Default|GetUpLocation)) _newtrack_0 1.0) false false)))))))

(event Game|Damage|EventAnyDamage
  (params (Damage :type Float%20%28single-precision%29) (DamageType :type Damage%20Type%20Object%20Reference) (InstigatedBy :type Controller%20Object%20Reference) (DamageCauser :type Actor%20Object%20Reference))
  (Class|FMODBlueprintStatics|PlayEvent2D "/Game/FMOD/Events/Enemies/Bosses/Monster_Punch.Monster_Punch"))

(event Collision|EventActorBeginOverlap
  (params (OtherActor :type Actor%20Object%20Reference)))

(event EventTick
  (params (DeltaSeconds :type Float%20%28single-precision%29)))

(event EventBeginPlay
  (bind _returnvalue (Rendering|Material|CreateDynamicMaterialInstance (Variables|Default|GetMiniMole) 0 "/Game/Assets/HumanHeads/ExWifeHead_Mat.ExWifeHead_Mat" "None" :!class /Script/Engine.PrimitiveComponent))
  (Variables|Default|SetBloodyMaterial _returnvalue)
  (Utilities|Time|SetTimerbyFunctionName 0 "GetUp" 0.1 true)
  (Utilities|Time|SetTimerbyFunctionName 0 "GetDown" 0.1 true 0.5))

(fn ConstructionScript)