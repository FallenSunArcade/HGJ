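; Mole enemy character that spawns when the player enters its detection sphere, then chases and catches them.
; It yaws toward the player each tick, and after a one-time spawn delay a looping timer re-issues AIMoveTo.
; Hand colliders trigger the player's caught sequence and stop movement, while a second sphere toggles Attacking.
; Damage depletes health until it sets DeadMole, disabling capsule collision and further move orders.
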(event OnComponentBeginOverlap(RangeDetectionSphere)
  (params (OverlappedComponent :type Primitive%20Component%20Object%20Reference) (OtherActor :type Actor%20Object%20Reference) (OtherComp :type Primitive%20Component%20Object%20Reference) (OtherBodyIndex :type Integer) (bFromSweep :type Boolean) (SweepResult :type Hit%20Result%20Structure%20%28by%20ref%29))
  (if (== (Utilities|Array|Get(acopy) (Variables|/Script/Engine.Actor|GetTags OtherActor)) "Player")
    (Utilities|FlowControl|DoOnce false
      (:Completed
        (Variables|Default|SetSpawn true)
        (Utilities|FlowControl|Delay 4.0)
        (Utilities|Time|SetTimerbyFunctionName 0 "FollowPlayer" 0.1 true)
        (Variables|Default|SetSpawn false)))))

(event OnComponentBeginOverlap(LefttHand_collider)
  (params (OverlappedComponent :type Primitive%20Component%20Object%20Reference) (OtherActor :type Actor%20Object%20Reference) (OtherComp :type Primitive%20Component%20Object%20Reference) (OtherBodyIndex :type Integer) (bFromSweep :type Boolean) (SweepResult :type Hit%20Result%20Structure%20%28by%20ref%29))
  ;[1 1 1] CatchPlayer
  (if (== (Utilities|Array|Get(acopy) (Variables|/Script/Engine.Actor|GetTags OtherActor)) "Player")
    (bind _asbp_player (Utilities|Casting|CastToBP_Player (Game|GetPlayerCharacter 0)))
    (Variables|/Game/BP_Player.BP_Player_C|SetCaught _asbp_player true)
    (Variables|Default|SetCatchPlayer true)
    (Variables|/Game/BP_Player.BP_Player_C|SetMonster _asbp_player self)
    (Default|GetsCaught _asbp_player)
    (Pawn|Components|CharacterMovement|SetMovementMode (Variables|Character|GetCharacterMovement) "MOVE_None" 0)))

(event OnComponentBeginOverlap(RightHand_collider)
  (params (OverlappedComponent :type Primitive%20Component%20Object%20Reference) (OtherActor :type Actor%20Object%20Reference) (OtherComp :type Primitive%20Component%20Object%20Reference) (OtherBodyIndex :type Integer) (bFromSweep :type Boolean) (SweepResult :type Hit%20Result%20Structure%20%28by%20ref%29))
  ;[1 1 1] CatchPlayer
  (if (== (Utilities|Array|Get(acopy) (Variables|/Script/Engine.Actor|GetTags OtherActor)) "Player")
    (bind _asbp_player (Utilities|Casting|CastToBP_Player (Game|GetPlayerCharacter 0)))
    (Variables|/Game/BP_Player.BP_Player_C|SetCaught _asbp_player true)
    (Variables|Default|SetCatchPlayer true)
    (Variables|/Game/BP_Player.BP_Player_C|SetMonster _asbp_player self)
    (Default|GetsCaught _asbp_player)
    (Pawn|Components|CharacterMovement|SetMovementMode (Variables|Character|GetCharacterMovement) "MOVE_None" 0)))

(event OnComponentBeginOverlap(RangeDetectionSphere1)
  (params (OverlappedComponent :type Primitive%20Component%20Object%20Reference) (OtherActor :type Actor%20Object%20Reference) (OtherComp :type Primitive%20Component%20Object%20Reference) (OtherBodyIndex :type Integer) (bFromSweep :type Boolean) (SweepResult :type Hit%20Result%20Structure%20%28by%20ref%29))
  (if (== (Utilities|Array|Get(acopy) (Variables|/Script/Engine.Actor|GetTags OtherActor)) "Player")
    (Variables|Default|SetAttacking true)))

(event OnComponentEndOverlap(RangeDetectionSphere1)
  (params (OverlappedComponent :type Primitive%20Component%20Object%20Reference) (OtherActor :type Actor%20Object%20Reference) (OtherComp :type Primitive%20Component%20Object%20Reference) (OtherBodyIndex :type Integer))
  (if (== (Utilities|Array|Get(acopy) (Variables|/Script/Engine.Actor|GetTags OtherActor)) "Player")
    (Variables|Default|SetAttacking false)))

(event Custom|FollowPlayer
  (if (not (Variables|Default|GetDeadMole))
    (AI|AIMoveTo self (Transformation|GetWorldLocation (Variables|/Script/Engine.Actor|GetRootComponent (Variables|Default|GetPlayer))) 0 3e+02 false)))

(event EventBeginPlay
  (bind _asbp_player (Utilities|Casting|CastToBP_Player (Game|GetPlayerCharacter 0)))
  (Variables|Default|SetPlayer _asbp_player))

(event EventTick
  (params (DeltaSeconds :type Float%20%28single-precision%29))
  (bind _returnvalue (Transformation|GetActorRotation))
  (if (not (Variables|Default|GetCatchPlayer))
    (Transformation|SetActorRotation (Math|Rotator|MakeRotator (.roll _returnvalue) (.pitch _returnvalue) (.yaw (Math|Rotator|FindLookatRotation (Transformation|GetActorLocation) (Transformation|GetActorLocation (Variables|Default|GetPlayer))))))))

(event Game|Damage|EventAnyDamage
  (params (Damage :type Float%20%28single-precision%29) (DamageType :type Damage%20Type%20Object%20Reference) (InstigatedBy :type Controller%20Object%20Reference) (DamageCauser :type Actor%20Object%20Reference))
  (bind _output_get (Variables|Default|SetMolehealth (- (Variables|Default|GetMolehealth) Damage)))
  (if (<= _output_get 0.0)
    (Variables|Default|SetDeadMole true)
    (Collision|SetCollisionEnabled (Variables|Collision|GetCapsuleComponent) "NoCollision")))

(fn ConstructionScript)