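; Flying duck boss minion that chases the player and deals contact damage.
; After a random delay it morphs via timeline-driven morph targets, rises, then a looping timer launches it toward the player while easing to their height.
; Player overlap triggers a DoOnce-gated hit and a launch in a random flee direction; leaving the outer capsule re-arms it.
; Roof-tagged components get knocked loose; any damage destroys it, leaving health-based death logic unconnected.
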(event OnComponentBeginOverlap(CollisionCapsule)
  (params (OverlappedComponent :type Primitive%20Component%20Object%20Reference) (OtherActor :type Actor%20Object%20Reference) (OtherComp :type Primitive%20Component%20Object%20Reference) (OtherBodyIndex :type Integer) (bFromSweep :type Boolean) (SweepResult :type Hit%20Result%20Structure%20%28by%20ref%29))
  (bind _returnvalue (Math|Random|RandomFloatinRange -3e+03 3e+03))
  (if (== (Utilities|Array|Get(acopy) (Variables|/Script/Engine.Actor|GetTags OtherActor)) "Player")
    (Utilities|FlowControl|DoOnce false
      (:Completed
        (if (not (Variables|Default|GetDead))
          (Game|Damage|ApplyDamage OtherActor 5.0 0 0)
          (if (not (Variables|Default|GetPlayerNearby))
            (Variables|Default|SetPlayerNearby true)
            (CallFunction|SwimAway)
            (bind _output_get (Variables|Default|SetFleePoint (Math|Vector|MakeVector _returnvalue _returnvalue (Math|Random|RandomFloatinRange 8e+02 1.2e+03))))
            (Variables|Default|SetFleePoint (Math|Vector|Normalize _output_get))))))
    (elif (== (Utilities|Array|Get(acopy) (Variables|/Script/Engine.ActorComponent|GetComponentTags OtherComp)) "roof")
      (bind _output_get_2 (Variables|Default|SetRoof OtherComp))
      (Physics|SetSimulatePhysics OtherComp true)
      (Physics|AddForce (Variables|Default|GetRoof) "30000.000000,30000.000000,30000.000000" "None" true))))

(event OnComponentEndOverlap(CollisionCapsule)
  (params (OverlappedComponent :type Primitive%20Component%20Object%20Reference) (OtherActor :type Actor%20Object%20Reference) (OtherComp :type Primitive%20Component%20Object%20Reference) (OtherBodyIndex :type Integer))
  (if (== (Utilities|Array|Get(acopy) (Variables|/Script/Engine.Actor|GetTags OtherActor)) "Player")
    _))

(event OnComponentBeginOverlap(AttackHitCollision)
  (params (OverlappedComponent :type Primitive%20Component%20Object%20Reference) (OtherActor :type Actor%20Object%20Reference) (OtherComp :type Primitive%20Component%20Object%20Reference) (OtherBodyIndex :type Integer) (bFromSweep :type Boolean) (SweepResult :type Hit%20Result%20Structure%20%28by%20ref%29))
  ;[1 1 1] PlayerHitable
  (if (== (Utilities|Array|Get(acopy) (Variables|/Script/Engine.Actor|GetTags OtherActor)) "Player")
    (Variables|Default|SetPlayerInAttackCollision true)))

(event OnComponentEndOverlap(AttackHitCollision)
  (params (OverlappedComponent :type Primitive%20Component%20Object%20Reference) (OtherActor :type Actor%20Object%20Reference) (OtherComp :type Primitive%20Component%20Object%20Reference) (OtherBodyIndex :type Integer))
  ;[1 1 1] PlayerHitable
  (if (== (Utilities|Array|Get(acopy) (Variables|/Script/Engine.Actor|GetTags OtherActor)) "Player")
    (Variables|Default|SetPlayerInAttackCollision false)))

(event OnComponentEndOverlap(CollisionCapsule1)
  (params (OverlappedComponent :type Primitive%20Component%20Object%20Reference) (OtherActor :type Actor%20Object%20Reference) (OtherComp :type Primitive%20Component%20Object%20Reference) (OtherBodyIndex :type Integer))
  (if (== (Utilities|Array|Get(acopy) (Variables|/Script/Engine.Actor|GetTags OtherActor)) "Player")
    (Variables|Default|SetPlayerNearby false)
    (CallFunction|ArrivedatFleepoint)))

(event OnComponentBeginOverlap(CollisionCapsule2)
  (params (OverlappedComponent :type Primitive%20Component%20Object%20Reference) (OtherActor :type Actor%20Object%20Reference) (OtherComp :type Primitive%20Component%20Object%20Reference) (OtherBodyIndex :type Integer) (bFromSweep :type Boolean) (SweepResult :type Hit%20Result%20Structure%20%28by%20ref%29))
  (Variables|Default|SetAttacking true))

(event OnComponentEndOverlap(CollisionCapsule2)
  (params (OverlappedComponent :type Primitive%20Component%20Object%20Reference) (OtherActor :type Actor%20Object%20Reference) (OtherComp :type Primitive%20Component%20Object%20Reference) (OtherBodyIndex :type Integer))
  (Variables|Default|SetAttacking false))

(event Custom|FollowPlayer
  ;[1 1 1] FollowPlayer
  (if (not (Variables|Default|GetDead))
    (if (Variables|Default|GetPlayerNearby)
      (CallFunction|SwimAway)
      (else
        (Variables|Default|SetFollowingPlayer true)
        (Character|LaunchCharacter (* (Math|Vector|Normalize (- (Transformation|GetActorLocation (Variables|Default|GetPlayer)) (Transformation|GetActorLocation))) (Variables|Default|GetSpeedNormal)) true true)
        (CallFunction|GetPlayerHight)))))

(event Custom|HitEnemy
  ;[1 1 1] PlayerHitable
)

(event Custom|ResetShapekeys)

(event Custom|Spawner
  (if (not (Variables|Default|GetSpawning))
    (bind _newtrack_0 (Timeline|Timeline PlayFromStart)
      (:Update
        (Components|SkeletalMesh|SetMorphTarget (Variables|Character|GetMesh) "longneck" _newtrack_0 true))
      (:Finished
        (bind _newtrack_0_2 (Timeline|Timeline_0 Play)
          (:Update
            (Components|SkeletalMesh|SetMorphTarget (Variables|Character|GetMesh) "beak" _newtrack_0_2 true))
          (:Finished
            (Variables|Default|SetSpawning true)
            (bind _newtrack_0_3 (Timeline|Timeline_1 PlayFromStart)
              (:Update
                (Components|SkeletalMesh|SetMorphTarget (Variables|Character|GetMesh) "layer 2" _newtrack_0_3 true)
                (Components|SkeletalMesh|SetMorphTarget (Variables|Character|GetMesh) "layer 3" _newtrack_0_3 true)
                (Components|SkeletalMesh|SetMorphTarget (Variables|Character|GetMesh) "layer 4" _newtrack_0_3 true))
              (:Finished
                (Utilities|FlowControl|Delay 3.0)
                (Timeline|Timeline_2 Play
                  (:Update
                    (Character|LaunchCharacter (+ "" "0.000000,0.000000,6.000000") false false))
                  (:Finished
                    (Utilities|Time|SetTimerbyFunctionName 0 "FollowPlayer" 0.5 true)
                    (Variables|Default|SetEvilSpawned true)))))))))))

(event Custom|StartFlying
  ;[1 1 1] RandomMovement
)

(event Custom|Rotate%20in%20Flying%20Direction
  (bind _returnvalue (Transformation|GetActorLocation))
  ;[1 1 1] RotateFish
  (if (Utilities|IsValid self)
    (bind _newtrack_0 (Timeline|Timeline_4 PlayFromStart)
      (:Update
        (Transformation|SetActorRotation (Math|Interpolation|RInterpTo (Transformation|GetActorRotation) (Math|Rotator|FindLookatRotation _returnvalue (+ _returnvalue (Variables|Default|GetLookRotation))) _newtrack_0 0.5))))))

(event Custom|RandomMovement
  ;[1 1 1] RandomMovement
)

(event Custom|GetPlayerHight
  (bind _returnvalue (Transformation|GetActorLocation))
  (bind _asbp_player (Utilities|Casting|CastToBP_Player (Game|GetPlayerCharacter 0)))
  (bind _newtrack_0 (Timeline|Timeline_10 PlayFromStart)
    (:Update
      (Transformation|SetActorLocation (Math|Vector|MakeVector (.x _returnvalue) (.y _returnvalue) (Math|Interpolation|FInterpTo (.z _returnvalue) (.z (Transformation|GetActorLocation _asbp_player)) _newtrack_0 1.0)) false false))))

(event Custom|SwimAway
  (bind _returnvalue (Transformation|GetActorLocation))
  ;[1 1 1] RandomMovement
  (CallFunction|GetPlayerHight)
  (if (Variables|Default|GetPlayerNearby)
    (if (not (Variables|Default|GetDead))
      (Character|LaunchCharacter (* (Variables|Default|GetFleePoint) (Variables|Default|GetDistanceToFlee)) true true)
      ;[1 1 1] RotateFish
      (bind _newtrack_0 (Timeline|Timeline_8 PlayFromStart)
        (:Update
          (Transformation|SetActorRotation (Math|Interpolation|RInterpTo (Transformation|GetActorRotation) (Math|Rotator|FindLookatRotation _returnvalue (+ _returnvalue (* (Variables|Default|GetFleePoint) (Variables|Default|GetDistanceToFlee)))) _newtrack_0 1e+01)))))))

(event Custom|ArrivedAtFleepoint
  (bind _returnvalue (Math|Random|RandomFloatinRange -3e+03 3e+03))
  (Utilities|FlowControl|DoOnce false) ; enters at Reset
)

(event EventBeginPlay
  (bind _asbp_player (Utilities|Casting|CastToBP_Player (Game|GetPlayerCharacter 0)))
  (Variables|Default|SetPlayer _asbp_player)
  (Utilities|FlowControl|Delay (Math|Random|RandomFloatinRange 0.0 3e+01))
  (Variables|Default|SetEvilSpawned true)
  (Utilities|FlowControl|DoOnce false
    (:Completed
      (bind _newtrack_0 (Timeline|Timeline PlayFromStart)
        (:Update
          (Components|SkeletalMesh|SetMorphTarget (Variables|Character|GetMesh) "longneck" _newtrack_0 true))
        (:Finished
          (bind _newtrack_0_2 (Timeline|Timeline_0 Play)
            (:Update
              (Components|SkeletalMesh|SetMorphTarget (Variables|Character|GetMesh) "beak" _newtrack_0_2 true))
            (:Finished
              (Variables|Default|SetSpawning true)
              (bind _newtrack_0_3 (Timeline|Timeline_1 PlayFromStart)
                (:Update
                  (Components|SkeletalMesh|SetMorphTarget (Variables|Character|GetMesh) "layer 2" _newtrack_0_3 true)
                  (Components|SkeletalMesh|SetMorphTarget (Variables|Character|GetMesh) "layer 3" _newtrack_0_3 true)
                  (Components|SkeletalMesh|SetMorphTarget (Variables|Character|GetMesh) "layer 4" _newtrack_0_3 true))
                (:Finished
                  (Utilities|FlowControl|Delay 3.0)
                  (Timeline|Timeline_2 Play
                    (:Update
                      (Character|LaunchCharacter (+ "" "0.000000,0.000000,6.000000") false false))
                    (:Finished
                      (Utilities|Time|SetTimerbyFunctionName 0 "FollowPlayer" 0.5 true)
                      (Variables|Default|SetEvilSpawned true))))))))))))

(event Game|Damage|EventAnyDamage
  (params (Damage :type Float%20%28single-precision%29) (DamageType :type Damage%20Type%20Object%20Reference) (InstigatedBy :type Controller%20Object%20Reference) (DamageCauser :type Actor%20Object%20Reference))
  ;[1 1 1] Damage+ Death
  (Actor|DestroyActor))

(event EventTick
  (params (DeltaSeconds :type Float%20%28single-precision%29))
  (bind _returnvalue (Transformation|GetActorLocation))
  (bind _player (Variables|Default|GetPlayer))
  (bind _returnvalue_2 (Transformation|GetActorLocation _player))
  (bind _returnvalue_3 (Math|Rotator|FindLookatRotation _returnvalue _returnvalue_2))
  ;[1 1 1] EventTick
  (if (Variables|Default|GetDead)
    (Transformation|SetActorLocation (+ (Transformation|GetActorLocation) "0.000000,0.000000,-50.000000") false false)
    (elif (Variables|Default|GetFollowingPlayer)
      (if (not (Variables|Default|GetPlayerNearby))
        (Transformation|SetActorRotation (Math|Interpolation|RInterpTo (Transformation|GetActorRotation) (Math|Rotator|MakeRotator (.roll _returnvalue_3) (.pitch _returnvalue_3) (.yaw _returnvalue_3)) (Utilities|Time|GetWorldDeltaSeconds) 3.0))))))

(fn ConstructionScript)