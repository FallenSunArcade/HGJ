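; Minion fish for the BOSS_Mother fight that morphs into an evil form and chases the player.
; BeginPlay randomizes capsule scale and starts chained morph-target timelines (player overlap can also trigger them), ending in a looping LaunchCharacter follow timer while Tick turns it toward the player.
; Any damage destroys it, updating the boss's shield: the last fish drops it during an active fight and makes Mother follow.
; Health-based death logic is disconnected.
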(event OnComponentBeginOverlap(CollisionCapsule)
  (params (OverlappedComponent :type Primitive%20Component%20Object%20Reference) (OtherActor :type Actor%20Object%20Reference) (OtherComp :type Primitive%20Component%20Object%20Reference) (OtherBodyIndex :type Integer) (bFromSweep :type Boolean) (SweepResult :type Hit%20Result%20Structure%20%28by%20ref%29))
  (if (== (Utilities|Array|Get(acopy) (Variables|/Script/Engine.Actor|GetTags OtherActor)) "Player")
    (if (Variables|Default|GetSpawning)
      (Variables|Default|SetPlayerNearby true)
      (bind _newtrack_0 (Timeline|Timeline Play)
        (:Update
          (Components|SkeletalMesh|SetMorphTarget (Variables|Character|GetMesh) "eyes2" _newtrack_0 true)
          (bind _newtrack_0_2 (Timeline|Timeline_0 Play)
            (:Update
              (Components|SkeletalMesh|SetMorphTarget (Variables|Character|GetMesh) "tail" _newtrack_0_2 true)
              (bind _newtrack_0_3 (Timeline|Timeline_3 Play)))
            (:Finished
              (bind _newtrack_0_4 (Timeline|Timeline_1 Play)
                (:Update
                  (Components|SkeletalMesh|SetMorphTarget (Variables|Character|GetMesh) "mouth" _newtrack_0_4 true)
                  (Components|SkeletalMesh|SetMorphTarget (Variables|Character|GetMesh) "mouth2" _newtrack_0_4 true))
                (:Finished
                  (bind _newtrack_0_5 (Timeline|Timeline_2 Play)
                    (:Update
                      (Components|SkeletalMesh|SetMorphTarget (Variables|Character|GetMesh) "teeth" _newtrack_0_5 true))
                    (:Finished
                      (Utilities|Time|SetTimerbyFunctionName 0 "FollowPlayer" 0.1 true)
                      (Variables|Default|SetSpawning false)
                      (Variables|Default|SetEvilSpawned true)))))))))
      (else
        (Variables|Default|SetSpawning true)
        (Timeline|Timeline Play)))))

(event OnComponentEndOverlap(CollisionCapsule)
  (params (OverlappedComponent :type Primitive%20Component%20Object%20Reference) (OtherActor :type Actor%20Object%20Reference) (OtherComp :type Primitive%20Component%20Object%20Reference) (OtherBodyIndex :type Integer))
  (if (== (Utilities|Array|Get(acopy) (Variables|/Script/Engine.Actor|GetTags OtherActor)) "Player")
    (Variables|Default|SetPlayerNearby false)))

(event OnComponentBeginOverlap(AttackHitCollision)
  (params (OverlappedComponent :type Primitive%20Component%20Object%20Reference) (OtherActor :type Actor%20Object%20Reference) (OtherComp :type Primitive%20Component%20Object%20Reference) (OtherBodyIndex :type Integer) (bFromSweep :type Boolean) (SweepResult :type Hit%20Result%20Structure%20%28by%20ref%29))
  ;[1 1 1] PlayerHitable
  (if (== (Utilities|Array|Get(acopy) (Variables|/Script/Engine.Actor|GetTags OtherActor)) "Player")
    (Variables|Default|SetPlayerInAttackCollision true)))

(event OnComponentEndOverlap(AttackHitCollision)
  (params (OverlappedComponent :type Primitive%20Component%20Object%20Reference) (OtherActor :type Actor%20Object%20Reference) (OtherComp :type Primitive%20Component%20Object%20Reference) (OtherBodyIndex :type Integer))
  ;[1 1 1] PlayerHitable
  (if (== (Utilities|Array|Get(acopy) (Variables|/Script/Engine.Actor|GetTags OtherActor)) "Player")
    (Variables|Default|SetPlayerInAttackCollision false)))

(event Custom|FollowPlayer
  ;[1 1 1] FollowPlayer
  (Character|LaunchCharacter (* (Math|Vector|Normalize (- (Transformation|GetActorLocation (Variables|Default|GetPlayer)) (Transformation|GetActorLocation))) (Variables|Default|GetSpeedNormal)) true true))

(event Custom|HitEnemy
  ;[1 1 1] PlayerHitable
  (Game|Damage|ApplyDamage (stale OnComponentBeginOverlap(AttackHitCollision) OtherActor) 5.0 0 0))

(event Custom|RandomMovement
  (bind _returnvalue (Transformation|GetActorLocation))
  ;[1 1 1] RandomMovement
  (if (not (Variables|Default|GetEvilSpawned))
    (if (not (Variables|Default|GetDead))
      (Variables|Default|SetLookRotation (Math|Vector|MakeVector (Math|Random|RandomFloatinRange -1.0 1.0) (Math|Random|RandomFloatinRange -1.0 1.0) (Math|Random|RandomFloatinRange -1.0 1.0)))
      (Character|LaunchCharacter (* (Variables|Default|GetLookRotation) (Variables|Default|GetSpeedNormal)) false false)
      ;[1 1 1] RotateFish
      (bind _newtrack_0 (Timeline|Timeline_4 PlayFromStart)
        (:Update
          (Transformation|SetActorRotation (Math|Interpolation|RInterpTo (Transformation|GetActorRotation) (Math|Rotator|FindLookatRotation _returnvalue (+ _returnvalue (Variables|Default|GetLookRotation))) _newtrack_0 0.5)))))))

(event EventBeginPlay
  (bind _returnvalue (Math|Random|RandomFloatinRange 0.8 2.0))
  (Transformation|SetWorldScale3D (Variables|Collision|GetCapsuleComponent) (Math|Vector|MakeVector _returnvalue _returnvalue _returnvalue))
  (Components|SkeletalMesh|SetMorphTarget (Variables|Character|GetMesh) "eyes" 1.0 true)
  (bind _asbp_player (Utilities|Casting|CastToBP_Player (Game|GetPlayerCharacter 0)))
  (Variables|Default|SetPlayer _asbp_player)
  (Development|PrintString "SPAWNINGFISH")
  (Variables|Default|SetSpawning true)
  (bind _newtrack_0 (Timeline|Timeline Play)
    (:Update
      (Components|SkeletalMesh|SetMorphTarget (Variables|Character|GetMesh) "eyes2" _newtrack_0 true)
      (bind _newtrack_0_2 (Timeline|Timeline_0 Play)
        (:Update
          (Components|SkeletalMesh|SetMorphTarget (Variables|Character|GetMesh) "tail" _newtrack_0_2 true)
          (bind _newtrack_0_3 (Timeline|Timeline_3 Play)))
        (:Finished
          (bind _newtrack_0_4 (Timeline|Timeline_1 Play)
            (:Update
              (Components|SkeletalMesh|SetMorphTarget (Variables|Character|GetMesh) "mouth" _newtrack_0_4 true)
              (Components|SkeletalMesh|SetMorphTarget (Variables|Character|GetMesh) "mouth2" _newtrack_0_4 true))
            (:Finished
              (bind _newtrack_0_5 (Timeline|Timeline_2 Play)
                (:Update
                  (Components|SkeletalMesh|SetMorphTarget (Variables|Character|GetMesh) "teeth" _newtrack_0_5 true))
                (:Finished
                  (Utilities|Time|SetTimerbyFunctionName 0 "FollowPlayer" 0.1 true)
                  (Variables|Default|SetSpawning false)
                  (Variables|Default|SetEvilSpawned true))))))))))

(event Game|Damage|EventAnyDamage
  (params (Damage :type Float%20%28single-precision%29) (DamageType :type Damage%20Type%20Object%20Reference) (InstigatedBy :type Controller%20Object%20Reference) (DamageCauser :type Actor%20Object%20Reference))
  (bind _asminion_fish_bp (Utilities|Casting|CastToMinion_Fish_BPClass "Minion_Fish_BP_C"))
  (bind _outactors (Actor|GetAllActorsOfClass _asminion_fish_bp))
  (if (< (Utilities|Array|Length _outactors) 2)
    (bind _asboss_mother (Utilities|Casting|CastToBOSS_MotherClass "/Game/Characters/Monster/BOSS_Versions/BOSS_Mother.BOSS_Mother_C"))
    (bind _returnvalue (Actor|GetActorOfClass _asboss_mother))
    (if (Variables|/Game/Characters/Monster/BOSS_Versions/BOSS_Mother.BOSS_Mother_C|GetBossfightHasStarted _returnvalue)
      (Variables|/Game/Characters/Monster/BOSS_Versions/BOSS_Mother.BOSS_Mother_C|SetShieldAvailable _returnvalue false)
      (Default|MotherFollowPlayer _returnvalue)
      (else
        (bind _asboss_mother_2 (Utilities|Casting|CastToBOSS_MotherClass "/Game/Characters/Monster/BOSS_Versions/BOSS_Mother.BOSS_Mother_C" :!label _label))
        (bind _returnvalue_2 (Actor|GetActorOfClass _asboss_mother_2))
        (Variables|/Game/Characters/Monster/BOSS_Versions/BOSS_Mother.BOSS_Mother_C|SetShieldAvailable _returnvalue_2 true)))
    (else
      (goto _label)))
  (Actor|DestroyActor))

(event EventTick
  (params (DeltaSeconds :type Float%20%28single-precision%29))
  (bind _returnvalue (Transformation|GetActorLocation))
  (bind _player (Variables|Default|GetPlayer))
  (bind _returnvalue_2 (Transformation|GetActorLocation _player))
  (bind _returnvalue_3 (Math|Rotator|FindLookatRotation _returnvalue _returnvalue_2))
  ;[1 1 1] EventTick
  (if (Variables|Default|GetDead)
    (Transformation|SetActorLocation (+ (Transformation|GetActorLocation) "0.000000,0.000000,5.000000") false false)
    (elif (Variables|Default|GetEvilSpawned)
      (Transformation|SetActorRotation (Math|Interpolation|RInterpTo (Transformation|GetActorRotation) (Math|Rotator|MakeRotator (.roll _returnvalue_3) (.pitch _returnvalue_3) (.yaw _returnvalue_3)) (Utilities|Time|GetWorldDeltaSeconds) 3.0)))))

(fn ConstructionScript)