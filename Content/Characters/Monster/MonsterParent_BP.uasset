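; Parent monster character that wakes when the player nears, then chases and catches them.
; AwakeCollision plays FMOD audio and starts a looping timer that reissues AIMoveTo toward the player until caught.
; Catch overlap notifies BP_Player and halts movement, while the attack volume only toggles AttackingPlayer.
; Damage drives a walk-speed timeline and, at zero health, staggered blood bursts; nested timelines animate mesh morph targets from BeginPlay.
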(event OnComponentBeginOverlap(PlayerCatchCollision)
  (params (OverlappedComponent :type Primitive%20Component%20Object%20Reference) (OtherActor :type Actor%20Object%20Reference) (OtherComp :type Primitive%20Component%20Object%20Reference) (OtherBodyIndex :type Integer) (bFromSweep :type Boolean) (SweepResult :type Hit%20Result%20Structure%20%28by%20ref%29))
  (bind _player (Variables|Default|GetPlayer))
  (if (not (Variables|Default|GetBigMonsterDead))
    (if (== (Utilities|Array|Get(acopy) (Variables|/Script/Engine.Actor|GetTags OtherActor)) "Player")
      (Variables|/Game/BP_Player.BP_Player_C|SetMonster _player self)
      (Variables|Default|SetCaughtPlayer true)
      (Variables|/Game/BP_Player.BP_Player_C|SetCaught _player true)
      (Default|GetsCaught _player)
      (Pawn|Components|CharacterMovement|SetMovementMode (Variables|Character|GetCharacterMovement) "MOVE_None" 0))))

(event OnComponentActivated(AIPerception)
  (params (Component :type Actor%20Component%20Object%20Reference) (bReset :type Boolean))
  (Development|PrintString "Perceived"))

(event OnComponentBeginOverlap(PlayerAttackCollision)
  (params (OverlappedComponent :type Primitive%20Component%20Object%20Reference) (OtherActor :type Actor%20Object%20Reference) (OtherComp :type Primitive%20Component%20Object%20Reference) (OtherBodyIndex :type Integer) (bFromSweep :type Boolean) (SweepResult :type Hit%20Result%20Structure%20%28by%20ref%29))
  (if (== (Utilities|Array|Get(acopy) (Variables|/Script/Engine.Actor|GetTags OtherActor)) "Player")
    (Variables|Default|SetAttackingPlayer true)))

(event OnComponentEndOverlap(PlayerAttackCollision)
  (params (OverlappedComponent :type Primitive%20Component%20Object%20Reference) (OtherActor :type Actor%20Object%20Reference) (OtherComp :type Primitive%20Component%20Object%20Reference) (OtherBodyIndex :type Integer))
  (if (== (Utilities|Array|Get(acopy) (Variables|/Script/Engine.Actor|GetTags OtherActor)) "Player")
    (Variables|Default|SetAttackingPlayer false)))

(event OnComponentBeginOverlap(AwakeCollision)
  (params (OverlappedComponent :type Primitive%20Component%20Object%20Reference) (OtherActor :type Actor%20Object%20Reference) (OtherComp :type Primitive%20Component%20Object%20Reference) (OtherBodyIndex :type Integer) (bFromSweep :type Boolean) (SweepResult :type Hit%20Result%20Structure%20%28by%20ref%29))
  (if (== (Utilities|Array|Get(acopy) (Variables|/Script/Engine.Actor|GetTags OtherActor)) "Player")
    (CallFunction|AwakeSound)
    (Variables|Default|SetAwake true)
    (Utilities|FlowControl|Delay 2.5)
    (Utilities|Time|SetTimerbyFunctionName 0 "FollowPlayer" 1.0 true)
    (Utilities|FlowControl|DoOnce false
      (:Completed
        (AddComponent|AddFMODAudioComponent false)))))

(event Custom|FollowPlayer
  (if (Variables|Default|GetAwake)
    (if (not (Variables|Default|GetCaughtPlayer))
      (AI|AIMoveTo self (Transformation|GetActorLocation (Variables|Default|GetPlayer)) 0 5.0 false))))

(event Custom|SlowDown
  (bind _newtrack_0 (Timeline|Timeline PlayFromStart)
    (:Update
      (Variables|/Script/Engine.CharacterMovementComponent|SetMaxWalkSpeed (Variables|Character|GetCharacterMovement) _newtrack_0))))

(event Custom|AwakeSound
  (Utilities|FlowControl|DoOnce false
    (:Completed
      (AddComponent|AddFMODAudioComponent false))))

(event EventBeginPlay
  (bind _asbp_player (Utilities|Casting|CastToBP_Player (Game|GetPlayerCharacter 0)))
  (Variables|Default|SetPlayer _asbp_player)
  (bind _newtrack_0 (Timeline|Timeline_0 Play)
    (:Update
      (Components|SkeletalMesh|SetMorphTarget (Variables|Character|GetMesh) "Key 1" _newtrack_0 true)
      (bind _newtrack_0_2 (Timeline|Timeline_1 Play)
        (:Update
          (Components|SkeletalMesh|SetMorphTarget (Variables|Character|GetMesh) "Key 2" _newtrack_0_2 true)
          (bind _newtrack_0_3 (Timeline|Timeline_2 Play)
            (:Update
              (Components|SkeletalMesh|SetMorphTarget (Variables|Character|GetMesh) "Key 4" _newtrack_0_3 true))))))))

(event Game|Damage|EventAnyDamage
  (params (Damage :type Float%20%28single-precision%29) (DamageType :type Damage%20Type%20Object%20Reference) (InstigatedBy :type Controller%20Object%20Reference) (DamageCauser :type Actor%20Object%20Reference))
  (CallFunction|SlowDown)
  (bind _output_get (Variables|Default|SetBigMonsterHealth (- (Variables|Default|GetBigMonsterHealth) Damage)))
  (if (<= _output_get 0.0)
    (Variables|Default|SetBigMonsterDead true)
    (Pawn|Components|CharacterMovement|SetMovementMode (Variables|Character|GetCharacterMovement) "MOVE_None" 0)
    (Collision|SetCollisionEnabled (Variables|Collision|GetCapsuleComponent) "NoCollision")
    (Effects|SpawnEmitteratLocation "/Game/Realistic_Starter_VFX_Pack_Vol2/Particles/Blood/P_Blood_Splat_Cone.P_Blood_Splat_Cone" (Transformation|GetActorLocation) (Math|Random|RandomRotator false))
    (Utilities|FlowControl|Delay 0.5)
    (Effects|SpawnEmitteratLocation "/Game/Realistic_Starter_VFX_Pack_Vol2/Particles/Blood/P_Blood_Splat_Cone.P_Blood_Splat_Cone" (+ (Transformation|GetActorLocation) "10.000000,-20.000000,20.000000") (Math|Random|RandomRotator false))
    (Utilities|FlowControl|Delay 0.5)
    (Effects|SpawnEmitteratLocation "/Game/Realistic_Starter_VFX_Pack_Vol2/Particles/Blood/P_Blood_Splat_Cone.P_Blood_Splat_Cone" (Transformation|GetActorLocation) (Math|Random|RandomRotator false))
    (Utilities|FlowControl|Delay 0.5)
    (Effects|SpawnEmitteratLocation "/Game/Realistic_Starter_VFX_Pack_Vol2/Particles/Blood/P_Blood_Splat_Cone.P_Blood_Splat_Cone" (+ (Transformation|GetActorLocation) "50.000000,-30.000000,50.000000") (Math|Random|RandomRotator false))
    (Utilities|FlowControl|Delay 0.5)
    (Effects|SpawnEmitteratLocation "/Game/Realistic_Starter_VFX_Pack_Vol2/Particles/Blood/P_Blood_Splat_Cone.P_Blood_Splat_Cone" (Transformation|GetActorLocation) (Math|Random|RandomRotator false))))

(fn ConstructionScript)