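; Randomized NPC that wanders until the player enters its R trigger, then permanently becomes a glowing-eyed zombie that follows the player.
; BeginPlay varies scale, body and face morph targets, and clothing colors through a dynamic material.
; Looping timers drive AI movement and FMOD mumbling, whose parameter changes on zombification and death, while chained timelines animate facial morphs.
; Damage drains health until death disables capsule collision; attack colliders only flag player overlap.
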(event OnComponentBeginOverlap(r)
  (params (OverlappedComponent :type Primitive%20Component%20Object%20Reference) (OtherActor :type Actor%20Object%20Reference) (OtherComp :type Primitive%20Component%20Object%20Reference) (OtherBodyIndex :type Integer) (bFromSweep :type Boolean) (SweepResult :type Hit%20Result%20Structure%20%28by%20ref%29))
  (if (== (Utilities|Array|Get(acopy) (Variables|/Script/Engine.Actor|GetTags OtherActor)) "Player")
    (Variables|Default|SetAttackingPlayer true)
    (CallFunction|BecomesZombie)))

(event OnComponentEndOverlap(r)
  (params (OverlappedComponent :type Primitive%20Component%20Object%20Reference) (OtherActor :type Actor%20Object%20Reference) (OtherComp :type Primitive%20Component%20Object%20Reference) (OtherBodyIndex :type Integer))
  (if (== (Utilities|Array|Get(acopy) (Variables|/Script/Engine.Actor|GetTags OtherActor)) "Player")
    (Variables|Default|SetAttackingPlayer false)))

(event OnComponentBeginOverlap(AttackCollider_L)
  (params (OverlappedComponent :type Primitive%20Component%20Object%20Reference) (OtherActor :type Actor%20Object%20Reference) (OtherComp :type Primitive%20Component%20Object%20Reference) (OtherBodyIndex :type Integer) (bFromSweep :type Boolean) (SweepResult :type Hit%20Result%20Structure%20%28by%20ref%29))
  (if (== (Utilities|Array|Get(acopy) (Variables|/Script/Engine.Actor|GetTags OtherActor)) "Player")
    (Variables|Default|SetColliderOverPlayer true)))

(event OnComponentEndOverlap(AttackCollider_L)
  (params (OverlappedComponent :type Primitive%20Component%20Object%20Reference) (OtherActor :type Actor%20Object%20Reference) (OtherComp :type Primitive%20Component%20Object%20Reference) (OtherBodyIndex :type Integer))
  (if (== (Utilities|Array|Get(acopy) (Variables|/Script/Engine.Actor|GetTags OtherActor)) "Player")
    (Variables|Default|SetColliderOverPlayer false)))

(event OnComponentBeginOverlap(AttackCollider_R)
  (params (OverlappedComponent :type Primitive%20Component%20Object%20Reference) (OtherActor :type Actor%20Object%20Reference) (OtherComp :type Primitive%20Component%20Object%20Reference) (OtherBodyIndex :type Integer) (bFromSweep :type Boolean) (SweepResult :type Hit%20Result%20Structure%20%28by%20ref%29))
  (if (== (Utilities|Array|Get(acopy) (Variables|/Script/Engine.Actor|GetTags OtherActor)) "Player")
    (Variables|Default|SetColliderOverPlayer true)))

(event OnComponentEndOverlap(AttackCollider_R)
  (params (OverlappedComponent :type Primitive%20Component%20Object%20Reference) (OtherActor :type Actor%20Object%20Reference) (OtherComp :type Primitive%20Component%20Object%20Reference) (OtherBodyIndex :type Integer))
  (if (== (Utilities|Array|Get(acopy) (Variables|/Script/Engine.Actor|GetTags OtherActor)) "Player")
    (Variables|Default|SetColliderOverPlayer false)))

(event Custom|NewShape
  (Variables|Default|SetRandomAnimationStart (Math|Random|RandomFloatinRange 1.2 0.8))
  (Transformation|SetWorldScale3D (Variables|Default|GetMan) (Math|Vector|MakeVector (Math|Random|RandomFloatinRange 0.75 0.85) (Math|Random|RandomFloatinRange 0.75 0.85) (Math|Random|RandomFloatinRange 0.65 0.85)))
  (Components|SkeletalMesh|SetMorphTarget (Variables|Default|GetMan) "fat" (Math|Random|RandomFloatinRange 0.0 1.0) true)
  (Components|SkeletalMesh|SetMorphTarget (Variables|Default|GetMan) "fit" (Math|Random|RandomFloatinRange 0.0 1.0) true)
  (Components|SkeletalMesh|SetMorphTarget (Variables|Default|GetMan) "Widehupperface" (Math|Random|RandomFloatinRange 0.0 1.0) true)
  (Components|SkeletalMesh|SetMorphTarget (Variables|Default|GetMan) "feninine" (Math|Random|RandomFloatinRange 0.0 1.0) true)
  (Components|SkeletalMesh|SetMorphTarget (Variables|Default|GetMan) "WideNose" (Math|Random|RandomFloatinRange 0.0 1.0) true)
  (Components|SkeletalMesh|SetMorphTarget (Variables|Default|GetMan) "StrongChin" (Math|Random|RandomFloatinRange -0.3 0.5) true)
  (Components|SkeletalMesh|SetMorphTarget (Variables|Default|GetMan) "longneck" (Math|Random|RandomFloatinRange 0.0 1.0) true)
  (Components|SkeletalMesh|SetMorphTarget (Variables|Default|GetMan) "earhight" (Math|Random|RandomFloatinRange 0.0 1.0) true)
  (Components|SkeletalMesh|SetMorphTarget (Variables|Default|GetMan) "eyehight" (Math|Random|RandomFloatinRange 0.0 1.0) true)
  (Components|SkeletalMesh|SetMorphTarget (Variables|Default|GetMan) "eyeangle" (Math|Random|RandomFloatinRange 0.0 1.0) true)
  (Components|SkeletalMesh|SetMorphTarget (Variables|Default|GetMan) "thickneck" (Math|Random|RandomFloatinRange 0.0 1.0) true)
  (Components|SkeletalMesh|SetMorphTarget (Variables|Default|GetMan) "nosebig" (Math|Random|RandomFloatinRange 0.0 1.0) true)
  (Components|SkeletalMesh|SetMorphTarget (Variables|Default|GetMan) "longnose" (Math|Random|RandomFloatinRange 0.0 1.0) true)
  (Components|SkeletalMesh|SetMorphTarget (Variables|Default|GetMan) "Hair2" (Math|Random|RandomFloatinRange 1.0 1.0) true)
  (Components|SkeletalMesh|SetMorphTarget (Variables|Default|GetMan) "Hair" (Math|Random|RandomFloatinRange 0.6 1.0) true)
  (Components|SkeletalMesh|SetMorphTarget (Variables|Default|GetMan) "hair3" (Math|Random|RandomFloatinRange 0.0 1.0) true)
  (bind _returnvalue (Rendering|Material|CreateDynamicMaterialInstance (Variables|Default|GetMan) 0 "/Game/Characters/Man/Textures/RandomMan_Mat.RandomMan_Mat" "None" :!class /Script/Engine.PrimitiveComponent))
  (bind _output_get (Variables|Default|SetMaterial _returnvalue))
  (Rendering|Material|SetScalarParameterValue _returnvalue "Shirt" 0.0 :!class /Script/Engine.MaterialInstanceDynamic)
  (if (Math|Random|RandomBool)
    (Rendering|Material|SetScalarParameterValue _returnvalue "Pants" 1.0 :!class /Script/Engine.MaterialInstanceDynamic)
    (else
      (Rendering|Material|SetScalarParameterValue _returnvalue "Pants" 0.0 :!class /Script/Engine.MaterialInstanceDynamic)))
  (Rendering|Material|SetVectorParameterValue _returnvalue "RandomColor" (Math|Conversions|ToLinearColor(Vector) (Math|Random|RandomUnitVector)) :!class /Script/Engine.MaterialInstanceDynamic)
  (if (< (Math|Random|RandomFloatinRange 1.0 0.0) 0.3)
    (if (Math|Random|RandomBool)
      (Rendering|Material|SetScalarParameterValue _returnvalue "Shirt" 2.0 :!class /Script/Engine.MaterialInstanceDynamic)
      (if (not (Math|Random|RandomBool)) :!label _label
        (if (Math|Random|RandomBool)
          (Rendering|Material|SetVectorParameterValue _returnvalue "RandomColor3" (Math|Conversions|ToLinearColor(Vector) (Math|Vector|MakeVector (Math|Random|RandomFloatinRange 1.0 0.0) (Math|Random|RandomFloatinRange 0.530423 0.0) (Math|Random|RandomFloatinRange 0.202043 0.0))) :!class /Script/Engine.MaterialInstanceDynamic))))
    (else
      (Rendering|Material|SetVectorParameterValue _returnvalue "RandomColor2" (Math|Conversions|ToLinearColor(Vector) (Math|Random|RandomUnitVector)) :!class /Script/Engine.MaterialInstanceDynamic)
      (goto _label))))

(event Custom|StopFaceAnim
  (bind _newtrack_0 (Timeline|Timeline Stop)
    (:Update
      (Components|SkeletalMesh|SetMorphTarget (Variables|Default|GetMan) "blink" _newtrack_0 true)
      (bind _newtrack_0_2 (Timeline|Timeline_0 Play)
        (:Update
          (Components|SkeletalMesh|SetMorphTarget (Variables|Default|GetMan) "angry" _newtrack_0_2 true)
          (bind _newtrack_0_3 (Timeline|Timeline_1 Play)
            (:Update
              (Components|SkeletalMesh|SetMorphTarget (Variables|Default|GetMan) "happy" _newtrack_0_3 true))))))))

(event Custom|Moving
  (if (not (Variables|Default|GetZombie))
    (if (not (Variables|Default|GetDead))
      (AI|AIMoveTo self (.RandomLocation (AI|Navigation|GetRandomReachablePointinRadius (Transformation|GetActorLocation) 1e+03 0 0)) 0 1e+02 true))))

(event Custom|BecomesZombie
  ;[1 1 1] Comment
  (Utilities|FlowControl|DoOnce false
    (:Completed
      (Variables|Default|SetMumbling_Man_FMOD 2.0)
      (Development|PrintString "Zombie")
      (Variables|Default|SetZombie true)
      (Utilities|Time|SetTimerbyFunctionName 0 "FollowPlayer" 0.5 true)
      (Rendering|Material|SetScalarParameterValue (Variables|Default|GetMaterial) "GlowingEyesParameter" 1.0 :!class /Script/Engine.MaterialInstanceDynamic))))

(event Custom|FollowPlayer
  (if (not (Variables|Default|GetDead))
    (bind _asbp_player (Utilities|Casting|CastToBP_Player (Game|GetPlayerCharacter 0)))
    (AI|AIMoveTo self (Transformation|GetActorLocation _asbp_player) 0 5.0 false)))

(event Custom|Begin%20Play1
  (Utilities|Time|SetTimerbyFunctionName 0 "Mumbling_Man" 6.0 true))

(event Custom|Mumbling_Man
  (bind _mumbling_man_fmod (Variables|Default|GetMumbling_Man_FMOD))
  (bind _returnvalue (Class|FMODBlueprintStatics|PlayEventatLocation "/Game/FMOD/Events/NPCs_Talking/Mumbling_Man_1.Mumbling_Man_1" (Math|Conversions|ToTransform(Vector) (Transformation|GetActorLocation))))
  (Class|FMODBlueprintStatics|EventInstancePlay _returnvalue)
  (bind _returnvalue_2 (Class|FMODBlueprintStatics|EventInstanceIsValid _returnvalue))
  (if _returnvalue_2
    (Class|FMODBlueprintStatics|EventInstanceSetParameter _returnvalue "Mumbling_Man_1" _mumbling_man_fmod)
    (Development|PrintString (Utilities|String|ToString(Float) _mumbling_man_fmod))))

(event EventBeginPlay
  (CallFunction|BeginPlay1)
  (Variables|Default|SetDeath12 (Math|Random|RandomBool))
  (Utilities|Time|SetTimerbyFunctionName 0 "Moving" (Math|Random|RandomFloatinRange 5.0 1e+01) true)
  (Variables|Default|SetRandomAnimationStart (Math|Random|RandomFloatinRange 1.2 0.8))
  (Transformation|SetWorldScale3D (Variables|Default|GetMan) (Math|Vector|MakeVector (Math|Random|RandomFloatinRange 0.75 0.85) (Math|Random|RandomFloatinRange 0.75 0.85) (Math|Random|RandomFloatinRange 0.65 0.85)))
  (Components|SkeletalMesh|SetMorphTarget (Variables|Default|GetMan) "fat" (Math|Random|RandomFloatinRange 0.0 1.0) true)
  (Components|SkeletalMesh|SetMorphTarget (Variables|Default|GetMan) "fit" (Math|Random|RandomFloatinRange 0.0 1.0) true)
  (Components|SkeletalMesh|SetMorphTarget (Variables|Default|GetMan) "Widehupperface" (Math|Random|RandomFloatinRange 0.0 1.0) true)
  (Components|SkeletalMesh|SetMorphTarget (Variables|Default|GetMan) "feninine" (Math|Random|RandomFloatinRange 0.0 1.0) true)
  (Components|SkeletalMesh|SetMorphTarget (Variables|Default|GetMan) "WideNose" (Math|Random|RandomFloatinRange 0.0 1.0) true)
  (Components|SkeletalMesh|SetMorphTarget (Variables|Default|GetMan) "StrongChin" (Math|Random|RandomFloatinRange -0.3 0.5) true)
  (Components|SkeletalMesh|SetMorphTarget (Variables|Default|GetMan) "longneck" (Math|Random|RandomFloatinRange 0.0 1.0) true)
  (Components|SkeletalMesh|SetMorphTarget (Variables|Default|GetMan) "earhight" (Math|Random|RandomFloatinRange 0.0 1.0) true)
  (Components|SkeletalMesh|SetMorphTarget (Variables|Default|GetMan) "eyehight" (Math|Random|RandomFloatinRange 0.0 1.0) true)
  (Components|SkeletalMesh|SetMorphTarget (Variables|Default|GetMan) "eyeangle" (Math|Random|RandomFloatinRange 0.0 1.0) true)
  (Components|SkeletalMesh|SetMorphTarget (Variables|Default|GetMan) "thickneck" (Math|Random|RandomFloatinRange 0.0 1.0) true)
  (Components|SkeletalMesh|SetMorphTarget (Variables|Default|GetMan) "nosebig" (Math|Random|RandomFloatinRange 0.0 1.0) true)
  (Components|SkeletalMesh|SetMorphTarget (Variables|Default|GetMan) "longnose" (Math|Random|RandomFloatinRange 0.0 1.0) true)
  (Components|SkeletalMesh|SetMorphTarget (Variables|Default|GetMan) "Hair2" (Math|Random|RandomFloatinRange 1.0 1.0) true)
  (Components|SkeletalMesh|SetMorphTarget (Variables|Default|GetMan) "Hair" (Math|Random|RandomFloatinRange 0.6 1.0) true)
  (Components|SkeletalMesh|SetMorphTarget (Variables|Default|GetMan) "hair3" (Math|Random|RandomFloatinRange 0.0 1.0) true)
  (bind _returnvalue (Rendering|Material|CreateDynamicMaterialInstance (Variables|Default|GetMan) 0 "/Game/Characters/Man/Textures/RandomMan_Mat.RandomMan_Mat" "None" :!class /Script/Engine.PrimitiveComponent))
  (bind _output_get (Variables|Default|SetMaterial _returnvalue))
  (Rendering|Material|SetScalarParameterValue _returnvalue "Shirt" 0.0 :!class /Script/Engine.MaterialInstanceDynamic)
  (if (Math|Random|RandomBool)
    (Rendering|Material|SetScalarParameterValue _returnvalue "Pants" 1.0 :!class /Script/Engine.MaterialInstanceDynamic)
    (else
      (Rendering|Material|SetScalarParameterValue _returnvalue "Pants" 0.0 :!class /Script/Engine.MaterialInstanceDynamic)))
  (Rendering|Material|SetVectorParameterValue _returnvalue "RandomColor" (Math|Conversions|ToLinearColor(Vector) (Math|Random|RandomUnitVector)) :!class /Script/Engine.MaterialInstanceDynamic)
  (if (< (Math|Random|RandomFloatinRange 1.0 0.0) 0.3)
    (if (Math|Random|RandomBool)
      (Rendering|Material|SetScalarParameterValue _returnvalue "Shirt" 2.0 :!class /Script/Engine.MaterialInstanceDynamic)
      (if (not (Math|Random|RandomBool)) :!label _label
        (if (Math|Random|RandomBool)
          (Rendering|Material|SetVectorParameterValue _returnvalue "RandomColor3" (Math|Conversions|ToLinearColor(Vector) (Math|Vector|MakeVector (Math|Random|RandomFloatinRange 1.0 0.0) (Math|Random|RandomFloatinRange 0.530423 0.0) (Math|Random|RandomFloatinRange 0.202043 0.0))) :!class /Script/Engine.MaterialInstanceDynamic))))
    (else
      (Rendering|Material|SetVectorParameterValue _returnvalue "RandomColor2" (Math|Conversions|ToLinearColor(Vector) (Math|Random|RandomUnitVector)) :!class /Script/Engine.MaterialInstanceDynamic)
      (goto _label))))

(event Collision|EventActorBeginOverlap
  (params (OtherActor :type Actor%20Object%20Reference)))

(event EventTick
  (params (DeltaSeconds :type Float%20%28single-precision%29))
  (bind _newtrack_0 (Timeline|Timeline Play)
    (:Update
      (Components|SkeletalMesh|SetMorphTarget (Variables|Default|GetMan) "blink" _newtrack_0 true)
      (bind _newtrack_0_2 (Timeline|Timeline_0 Play)
        (:Update
          (Components|SkeletalMesh|SetMorphTarget (Variables|Default|GetMan) "angry" _newtrack_0_2 true)
          (bind _newtrack_0_3 (Timeline|Timeline_1 Play)
            (:Update
              (Components|SkeletalMesh|SetMorphTarget (Variables|Default|GetMan) "happy" _newtrack_0_3 true))))))))

(event Game|Damage|EventAnyDamage
  (params (Damage :type Float%20%28single-precision%29) (DamageType :type Damage%20Type%20Object%20Reference) (InstigatedBy :type Controller%20Object%20Reference) (DamageCauser :type Actor%20Object%20Reference))
  (Variables|Default|SetRandomNPCHealth (- (Variables|Default|GetRandomNPCHealth) Damage))
  (if (<= (Variables|Default|GetRandomNPCHealth) 0.0)
    (Variables|Default|SetDead true)
    (Collision|SetCollisionEnabled (Variables|Collision|GetCapsuleComponent) "NoCollision")
    (CallFunction|StopFaceAnim)
    (Variables|Default|SetMumbling_Man_FMOD 0.0)))

(fn ConstructionScript)