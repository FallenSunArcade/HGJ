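; Seated mother character that animates facial expressions on the Mother3 mesh through morph targets.
; BeginPlay applies fixed mother, breasts, shirt and size morphs to set the body shape.
; Tick plays a chain of three timelines, each update starting the next, to drive eyesclosed, eyessmall and happy.
; Randomization of scale, face, hair and material colors is left disconnected and never runs, and NewShape is empty.
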(event Custom|NewShape)

(event Collision|EventActorBeginOverlap
  (params (OtherActor :type Actor%20Object%20Reference)))

(event EventTick
  (params (DeltaSeconds :type Float%20%28single-precision%29))
  (bind _newtrack_0 (Timeline|Timeline Play)
    (:Update
      (Components|SkeletalMesh|SetMorphTarget (Variables|Default|Getmother3) "eyesclosed" _newtrack_0 true)
      (bind _newtrack_0_2 (Timeline|Timeline_0 Play)
        (:Update
          (Components|SkeletalMesh|SetMorphTarget (Variables|Default|Getmother3) "eyessmall" _newtrack_0_2 true)
          (bind _newtrack_0_3 (Timeline|Timeline_1 Play)
            (:Update
              (Components|SkeletalMesh|SetMorphTarget (Variables|Default|Getmother3) "happy" _newtrack_0_3 true))))))))

(event EventBeginPlay
  (Components|SkeletalMesh|SetMorphTarget (Variables|Default|Getmother3) "mother" 1.0 true)
  (Components|SkeletalMesh|SetMorphTarget (Variables|Default|Getmother3) "breasts" 1.0 true)
  (Components|SkeletalMesh|SetMorphTarget (Variables|Default|Getmother3) "shirt" 1.0 true)
  (Components|SkeletalMesh|SetMorphTarget (Variables|Default|Getmother3) "size" 0.5 true))

(fn ConstructionScript)