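; RandomWoman_BP is an NPC woman who wanders to random nearby points and turns into a player-chasing zombie when the player overlaps her R component.
; BeginPlay and NewShape randomize scale, morph targets and dynamic material clothing parameters for a varied look.
; Tick drives nested face-morph timelines, while looping timers issue wander and chase moves.
; Attack colliders only set overlap flags; any damage marks her dead, disabling capsule collision.
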(event OnComponentBeginOverlap(r)
  (params (OverlappedComponent :type Primitive%20Component%20Object%20Reference) (OtherActor :type Actor%20Object%20Reference) (OtherComp :type Primitive%20Component%20Object%20Reference) (OtherBodyIndex :type Integer) (bFromSweep :type Boolean) (SweepResult :type Hit%20Result%20Structure%20%28by%20ref%29))
  (if (== (Utilities|Array|Get(acopy) (Variables|/Script/Engine.Actor|GetTags OtherActor)) "Player")
    (Variables|Default|SetAttackingPlayer true)
    (CallFunction|BecomesZombie)))

(event OnComponentEndOverlap(r)
  (params (OverlappedComponent :type Primitive%20Component%20Object%20Reference) (OtherActor :type Actor%20Object%20Reference) (OtherComp :type Primitive%20Component%20Object%20Reference) (OtherBodyIndex :type Integer))
  (if (== (Utilities|Array|Get(acopy) (Variables|/Script/Engine.Actor|GetTags OtherActor)) "Player")
    (Variables|Default|SetAttackingPlayer false)))

(event OnComponentBeginOverlap(AttackCollider_L)
  (params (OverlappedComponent :type Primitive%20Component%20Object%20Reference) (OtherActor :type Actor%20Object%20Reference) (OtherComp :type Primitive%20Component%20Object%20Reference) (OtherBodyIndex :type Integer) (bFromSweep :type Boolean) (SweepResult :type Hit%20Result%20Structure%20%28by%20ref%29))
  (if (== (Utilities|Array|Get(acopy) (Variables|/Script/Engine.Actor|GetTags OtherActor)) "Player")
    (Variables|Default|SetColliderOverPlayer true)))

(event OnComponentEndOverlap(AttackCollider_L)
  (params (OverlappedComponent :type Primitive%20Component%20Object%20Reference) (OtherActor :type Actor%20Object%20Reference) (OtherComp :type Primitive%20Component%20Object%20Reference) (OtherBodyIndex :type Integer))
  (if (== (Utilities|Array|Get(acopy) (Variables|/Script/Engine.Actor|GetTags OtherActor)) "Player")
    (Variables|Default|SetColliderOverPlayer false)))

(event OnComponentBeginOverlap(AttackCollider_R)
  (params (OverlappedComponent :type Primitive%20Component%20Object%20Reference) (OtherActor :type Actor%20Object%20Reference) (OtherComp :type Primitive%20Component%20Object%20Reference) (OtherBodyIndex :type Integer) (bFromSweep :type Boolean) (SweepResult :type Hit%20Result%20Structure%20%28by%20ref%29))
  (if (== (Utilities|Array|Get(acopy) (Variables|/Script/Engine.Actor|GetTags OtherActor)) "Player")
    (Variables|Default|SetAttackingPlayer true)))

(event OnComponentEndOverlap(AttackCollider_R)
  (params (OverlappedComponent :type Primitive%20Component%20Object%20Reference) (OtherActor :type Actor%20Object%20Reference) (OtherComp :type Primitive%20Component%20Object%20Reference) (OtherBodyIndex :type Integer))
  (if (== (Utilities|Array|Get(acopy) (Variables|/Script/Engine.Actor|GetTags OtherActor)) "Player")
    (Variables|Default|SetAttackingPlayer false)))

(event Custom|NewShape
  (Variables|Default|SetRandomAnimationStart (Math|Random|RandomFloatinRange 1.2 0.8))
  (Transformation|SetWorldScale3D (Variables|Default|Getwoman) (Math|Vector|MakeVector (Math|Random|RandomFloatinRange 0.65 0.7) (Math|Random|RandomFloatinRange 0.65 0.7) (Math|Random|RandomFloatinRange 0.55 0.7)))
  (Components|SkeletalMesh|SetMorphTarget (Variables|Default|Getwoman) "size" (Math|Random|RandomFloatinRange 0.0 1.0) true)
  (Components|SkeletalMesh|SetMorphTarget (Variables|Default|Getwoman) "breasts" (Math|Random|RandomFloatinRange 0.0 1.0) true)
  (Components|SkeletalMesh|SetMorphTarget (Variables|Default|Getwoman) "shirt" (Math|Random|RandomFloatinRange 0.0 1.0) true)
  (Components|SkeletalMesh|SetMorphTarget (Variables|Default|Getwoman) "feet" (Math|Random|RandomFloatinRange 0.0 1.0) true)
  (Components|SkeletalMesh|SetMorphTarget (Variables|Default|Getwoman) "neck" (Math|Random|RandomFloatinRange 0.0 1.0) true)
  (Components|SkeletalMesh|SetMorphTarget (Variables|Default|Getwoman) "pointyshoe" (Math|Random|RandomFloatinRange 0.0 1.0) true)
  (Components|SkeletalMesh|SetMorphTarget (Variables|Default|Getwoman) "Happy" (Math|Random|RandomFloatinRange 0.0 1.0) true)
  (Components|SkeletalMesh|SetMorphTarget (Variables|Default|Getwoman) "Sad" (Math|Random|RandomFloatinRange 0.0 0.5) true)
  (Components|SkeletalMesh|SetMorphTarget (Variables|Default|Getwoman) "angry" (Math|Random|RandomFloatinRange 0.0 1.0) true)
  (Components|SkeletalMesh|SetMorphTarget (Variables|Default|Getwoman) "dress" (Math|Random|RandomFloatinRange 0.0 1.0) true)
  (Components|SkeletalMesh|SetMorphTarget (Variables|Default|Getwoman) "FaceShape" (Math|Random|RandomFloatinRange 0.0 0.3) true)
  (Components|SkeletalMesh|SetMorphTarget (Variables|Default|Getwoman) "Key 19" (Math|Random|RandomFloatinRange 0.0 0.3) true)
  (Components|SkeletalMesh|SetMorphTarget (Variables|Default|Getwoman) "Key 20" (Math|Random|RandomFloatinRange 0.0 0.3) true)
  (Components|SkeletalMesh|SetMorphTarget (Variables|Default|Getwoman) "Key 21" (Math|Random|RandomFloatinRange 0.0 0.3) true)
  (Components|SkeletalMesh|SetMorphTarget (Variables|Default|Getwoman) "Key 22" (Math|Random|RandomFloatinRange 0.0 0.3) true)
  (Components|SkeletalMesh|SetMorphTarget (Variables|Default|Getwoman) "Key 23" (Math|Random|RandomFloatinRange 0.0 0.3) true)
  (Components|SkeletalMesh|SetMorphTarget (Variables|Default|Getwoman) "Key 24" (Math|Random|RandomFloatinRange 0.0 0.3) true)
  (Components|SkeletalMesh|SetMorphTarget (Variables|Default|Getwoman) "Key 25" (Math|Random|RandomFloatinRange 0.0 0.3) true)
  (Components|SkeletalMesh|SetMorphTarget (Variables|Default|Getwoman) "Key 26" (Math|Random|RandomFloatinRange 0.0 0.3) true)
  (Components|SkeletalMesh|SetMorphTarget (Variables|Default|Getwoman) "Key 27" (Math|Random|RandomFloatinRange 0.0 0.3) true)
  (Components|SkeletalMesh|SetMorphTarget (Variables|Default|Getwoman) "Key 28" (Math|Random|RandomFloatinRange 0.0 0.3) true)
  (Components|SkeletalMesh|SetMorphTarget (Variables|Default|Getwoman) "Key 29" (Math|Random|RandomFloatinRange 0.0 0.3) true)
  (Components|SkeletalMesh|SetMorphTarget (Variables|Default|Getwoman) "Key 30" (Math|Random|RandomFloatinRange 0.0 0.3) true)
  (Components|SkeletalMesh|SetMorphTarget (Variables|Default|Getwoman) "Key 31" (Math|Random|RandomFloatinRange 0.0 0.3) true)
  (Components|SkeletalMesh|SetMorphTarget (Variables|Default|Getwoman) "Key 32" (Math|Random|RandomFloatinRange 0.0 0.3) true)
  (Components|SkeletalMesh|SetMorphTarget (Variables|Default|Getwoman) "Key 33" (Math|Random|RandomFloatinRange 0.0 0.3) true)
  (Components|SkeletalMesh|SetMorphTarget (Variables|Default|Getwoman) "Key 34" (Math|Random|RandomFloatinRange 0.0 0.13) true)
  (Components|SkeletalMesh|SetMorphTarget (Variables|Default|Getwoman) "Key 35" (Math|Random|RandomFloatinRange 0.0 1.0) true)
  (Components|SkeletalMesh|SetMorphTarget (Variables|Default|Getwoman) "Key 36" (Math|Random|RandomFloatinRange 0.0 1.0) true)
  (if (< (Math|Random|RandomFloatinRange 0.0 1.0) 0.5)
    (Components|SkeletalMesh|SetMorphTarget (Variables|Default|Getwoman) "hair1" 0.0 true))
  (Components|SkeletalMesh|SetMorphTarget (Variables|Default|Getwoman) "hair2" (Math|Random|RandomFloatinRange 0.0 1.0) true)
  (Components|SkeletalMesh|SetMorphTarget (Variables|Default|Getwoman) "hair2B" (Math|Random|RandomFloatinRange 0.0 1.0) true)
  (bind _returnvalue (Rendering|Material|CreateDynamicMaterialInstance (Variables|Default|Getwoman) 0 "/Game/Characters/Woman/Woman_Mat.Woman_Mat" "None" :!class /Script/Engine.PrimitiveComponent))
  (Variables|Default|SetMaterial _returnvalue)
  (if (< (Math|Random|RandomFloatinRange 0.0 1.0) 0.2)
    (Rendering|Material|SetScalarParameterValue _returnvalue "Shirt" 1.0 :!class /Script/Engine.MaterialInstanceDynamic)
    (else
      (Rendering|Material|SetScalarParameterValue _returnvalue "Shirt" 0.0 :!class /Script/Engine.MaterialInstanceDynamic)))
  (if (Math|Random|RandomBool)
    (Rendering|Material|SetScalarParameterValue _returnvalue "Pants" 1.0 :!class /Script/Engine.MaterialInstanceDynamic)
    (else
      (Rendering|Material|SetScalarParameterValue _returnvalue "Pants" 0.0 :!class /Script/Engine.MaterialInstanceDynamic)))
  (Rendering|Material|SetVectorParameterValue _returnvalue "RandomColor" (Math|Conversions|ToLinearColor(Vector) (Math|Random|RandomUnitVector)) :!class /Script/Engine.MaterialInstanceDynamic)
  (if (< (Math|Random|RandomFloatinRange 1.0 0.0) 0.3)
    (if (Math|Random|RandomBool)
      (Rendering|Material|SetScalarParameterValue _returnvalue "Shirt" 2.0 :!class /Script/Engine.MaterialInstanceDynamic)
      (Development|PrintString "Hello")
      (if (not (Math|Random|RandomBool)) :!label _label
        (if (Math|Random|RandomBool)
          (Rendering|Material|SetVectorParameterValue _returnvalue "RandomColor3" (Math|Conversions|ToLinearColor(Vector) (Math|Vector|MakeVector (Math|Random|RandomFloatinRange 1.0 0.0) (Math|Random|RandomFloatinRange 0.530423 0.0) (Math|Random|RandomFloatinRange 0.202043 0.0))) :!class /Script/Engine.MaterialInstanceDynamic))))
    (else
      (Rendering|Material|SetVectorParameterValue _returnvalue "RandomColor2" (Math|Conversions|ToLinearColor(Vector) (Math|Random|RandomUnitVector)) :!class /Script/Engine.MaterialInstanceDynamic)
      (goto _label))))

(event Custom|StopFaceAnim
  (bind _newtrack_0 (Timeline|Timeline Stop)
    (:Update
      (Components|SkeletalMesh|SetMorphTarget (Variables|Default|Getwoman) "eyesclosed" _newtrack_0 true)
      (bind _newtrack_0_2 (Timeline|Timeline_0 Play)
        (:Update
          (Components|SkeletalMesh|SetMorphTarget (Variables|Default|Getwoman) "eyessmall" _newtrack_0_2 true)
          (bind _newtrack_0_3 (Timeline|Timeline_1 Play)
            (:Update
              (Components|SkeletalMesh|SetMorphTarget (Variables|Default|Getwoman) "happy" _newtrack_0_3 true))))))))

(event Custom|Moving
  (if (not (Variables|Default|GetStatic?))
    (bind _asbp_player (Utilities|Casting|CastToBP_Player (Game|GetPlayerCharacter 0)))
    (if (not (Variables|Default|GetDead))
      (AI|AIMoveTo self (.RandomLocation (AI|Navigation|GetRandomReachablePointinRadius (Transformation|GetActorLocation) 1e+03 0 0)) 0 1e+02 true))))

(event Custom|FollowPlayer
  (if (not (Variables|Default|GetStatic?))
    (if (not (Variables|Default|GetDead))
      (bind _asbp_player (Utilities|Casting|CastToBP_Player (Game|GetPlayerCharacter 0)))
      (AI|AIMoveTo self (Transformation|GetActorLocation _asbp_player) 0 5.0 false))))

(event Custom|BecomesZombie
  ;[1 1 1] Comment
  (Development|PrintString "Zombie")
  (Variables|Default|SetZombie true)
  (Utilities|Time|SetTimerbyFunctionName 0 "FollowPlayer" 0.5 true))

(event EventBeginPlay
  (Variables|Default|SetDeath12 (Math|Random|RandomBool))
  (Utilities|Time|SetTimerbyFunctionName 0 "Moving" (Math|Random|RandomFloatinRange 5.0 1e+01) true)
  (Variables|Default|SetRandomAnimationStart (Math|Random|RandomFloatinRange 1.2 0.8))
  (Transformation|SetWorldScale3D (Variables|Default|Getwoman) (Math|Vector|MakeVector (Math|Random|RandomFloatinRange 0.65 0.7) (Math|Random|RandomFloatinRange 0.65 0.7) (Math|Random|RandomFloatinRange 0.55 0.7)))
  (Components|SkeletalMesh|SetMorphTarget (Variables|Default|Getwoman) "size" (Math|Random|RandomFloatinRange 0.0 1.0) true)
  (Components|SkeletalMesh|SetMorphTarget (Variables|Default|Getwoman) "breasts" (Math|Random|RandomFloatinRange 0.0 1.0) true)
  (Components|SkeletalMesh|SetMorphTarget (Variables|Default|Getwoman) "shirt" (Math|Random|RandomFloatinRange 0.0 1.0) true)
  (Components|SkeletalMesh|SetMorphTarget (Variables|Default|Getwoman) "feet" (Math|Random|RandomFloatinRange 0.0 1.0) true)
  (Components|SkeletalMesh|SetMorphTarget (Variables|Default|Getwoman) "neck" (Math|Random|RandomFloatinRange 0.0 1.0) true)
  (Components|SkeletalMesh|SetMorphTarget (Variables|Default|Getwoman) "pointyshoe" (Math|Random|RandomFloatinRange 0.0 1.0) true)
  (Components|SkeletalMesh|SetMorphTarget (Variables|Default|Getwoman) "Happy" (Math|Random|RandomFloatinRange 0.0 1.0) true)
  (Components|SkeletalMesh|SetMorphTarget (Variables|Default|Getwoman) "Sad" (Math|Random|RandomFloatinRange 0.0 0.5) true)
  (Components|SkeletalMesh|SetMorphTarget (Variables|Default|Getwoman) "angry" (Math|Random|RandomFloatinRange 0.0 1.0) true)
  (Components|SkeletalMesh|SetMorphTarget (Variables|Default|Getwoman) "dress" (Math|Random|RandomFloatinRange 0.0 1.0) true)
  (Components|SkeletalMesh|SetMorphTarget (Variables|Default|Getwoman) "FaceShape" (Math|Random|RandomFloatinRange 0.0 0.3) true)
  (Components|SkeletalMesh|SetMorphTarget (Variables|Default|Getwoman) "Key 19" (Math|Random|RandomFloatinRange 0.0 0.3) true)
  (Components|SkeletalMesh|SetMorphTarget (Variables|Default|Getwoman) "Key 20" (Math|Random|RandomFloatinRange 0.0 0.3) true)
  (Components|SkeletalMesh|SetMorphTarget (Variables|Default|Getwoman) "Key 21" (Math|Random|RandomFloatinRange 0.0 0.3) true)
  (Components|SkeletalMesh|SetMorphTarget (Variables|Default|Getwoman) "Key 22" (Math|Random|RandomFloatinRange 0.0 0.3) true)
  (Components|SkeletalMesh|SetMorphTarget (Variables|Default|Getwoman) "Key 23" (Math|Random|RandomFloatinRange 0.0 0.3) true)
  (Components|SkeletalMesh|SetMorphTarget (Variables|Default|Getwoman) "Key 24" (Math|Random|RandomFloatinRange 0.0 0.3) true)
  (Components|SkeletalMesh|SetMorphTarget (Variables|Default|Getwoman) "Key 25" (Math|Random|RandomFloatinRange 0.0 0.3) true)
  (Components|SkeletalMesh|SetMorphTarget (Variables|Default|Getwoman) "Key 26" (Math|Random|RandomFloatinRange 0.0 0.3) true)
  (Components|SkeletalMesh|SetMorphTarget (Variables|Default|Getwoman) "Key 27" (Math|Random|RandomFloatinRange 0.0 0.3) true)
  (Components|SkeletalMesh|SetMorphTarget (Variables|Default|Getwoman) "Key 28" (Math|Random|RandomFloatinRange 0.0 0.3) true)
  (Components|SkeletalMesh|SetMorphTarget (Variables|Default|Getwoman) "Key 29" (Math|Random|RandomFloatinRange 0.0 0.3) true)
  (Components|SkeletalMesh|SetMorphTarget (Variables|Default|Getwoman) "Key 30" (Math|Random|RandomFloatinRange 0.0 0.3) true)
  (Components|SkeletalMesh|SetMorphTarget (Variables|Default|Getwoman) "Key 31" (Math|Random|RandomFloatinRange 0.0 0.3) true)
  (Components|SkeletalMesh|SetMorphTarget (Variables|Default|Getwoman) "Key 32" (Math|Random|RandomFloatinRange 0.0 0.3) true)
  (Components|SkeletalMesh|SetMorphTarget (Variables|Default|Getwoman) "Key 33" (Math|Random|RandomFloatinRange 0.0 0.3) true)
  (Components|SkeletalMesh|SetMorphTarget (Variables|Default|Getwoman) "Key 34" (Math|Random|RandomFloatinRange 0.0 0.13) true)
  (Components|SkeletalMesh|SetMorphTarget (Variables|Default|Getwoman) "Key 35" (Math|Random|RandomFloatinRange 0.0 1.0) true)
  (Components|SkeletalMesh|SetMorphTarget (Variables|Default|Getwoman) "Key 36" (Math|Random|RandomFloatinRange 0.0 1.0) true)
  (if (< (Math|Random|RandomFloatinRange 0.0 1.0) 0.5)
    (Components|SkeletalMesh|SetMorphTarget (Variables|Default|Getwoman) "hair1" 0.0 true))
  (Components|SkeletalMesh|SetMorphTarget (Variables|Default|Getwoman) "hair2" (Math|Random|RandomFloatinRange 0.0 1.0) true)
  (Components|SkeletalMesh|SetMorphTarget (Variables|Default|Getwoman) "hair2B" (Math|Random|RandomFloatinRange 0.0 1.0) true)
  (bind _returnvalue (Rendering|Material|CreateDynamicMaterialInstance (Variables|Default|Getwoman) 0 "/Game/Characters/Woman/Woman_Mat.Woman_Mat" "None" :!class /Script/Engine.PrimitiveComponent))
  (Variables|Default|SetMaterial _returnvalue)
  (if (< (Math|Random|RandomFloatinRange 0.0 1.0) 0.2)
    (Rendering|Material|SetScalarParameterValue _returnvalue "Shirt" 1.0 :!class /Script/Engine.MaterialInstanceDynamic)
    (else
      (Rendering|Material|SetScalarParameterValue _returnvalue "Shirt" 0.0 :!class /Script/Engine.MaterialInstanceDynamic)))
  (if (Math|Random|RandomBool)
    (Rendering|Material|SetScalarParameterValue _returnvalue "Pants" 1.0 :!class /Script/Engine.MaterialInstanceDynamic)
    (else
      (Rendering|Material|SetScalarParameterValue _returnvalue "Pants" 0.0 :!class /Script/Engine.MaterialInstanceDynamic)))
  (Rendering|Material|SetVectorParameterValue _returnvalue "RandomColor" (Math|Conversions|ToLinearColor(Vector) (Math|Random|RandomUnitVector)) :!class /Script/Engine.MaterialInstanceDynamic)
  (if (< (Math|Random|RandomFloatinRange 1.0 0.0) 0.3)
    (if (Math|Random|RandomBool)
      (Rendering|Material|SetScalarParameterValue _returnvalue "Shirt" 2.0 :!class /Script/Engine.MaterialInstanceDynamic)
      (Development|PrintString "Hello")
      (if (not (Math|Random|RandomBool)) :!label _label
        (if (Math|Random|RandomBool)
          (Rendering|Material|SetVectorParameterValue _returnvalue "RandomColor3" (Math|Conversions|ToLinearColor(Vector) (Math|Vector|MakeVector (Math|Random|RandomFloatinRange 1.0 0.0) (Math|Random|RandomFloatinRange 0.530423 0.0) (Math|Random|RandomFloatinRange 0.202043 0.0))) :!class /Script/Engine.MaterialInstanceDynamic))))
    (else
      (Rendering|Material|SetVectorParameterValue _returnvalue "RandomColor2" (Math|Conversions|ToLinearColor(Vector) (Math|Random|RandomUnitVector)) :!class /Script/Engine.MaterialInstanceDynamic)
      (goto _label))))

(event Collision|EventActorBeginOverlap
  (params (OtherActor :type Actor%20Object%20Reference)))

(event EventTick
  (params (DeltaSeconds :type Float%20%28single-precision%29))
  (bind _newtrack_0 (Timeline|Timeline Play)
    (:Update
      (Components|SkeletalMesh|SetMorphTarget (Variables|Default|Getwoman) "eyesclosed" _newtrack_0 true)
      (bind _newtrack_0_2 (Timeline|Timeline_0 Play)
        (:Update
          (Components|SkeletalMesh|SetMorphTarget (Variables|Default|Getwoman) "eyessmall" _newtrack_0_2 true)
          (bind _newtrack_0_3 (Timeline|Timeline_1 Play)
            (:Update
              (Components|SkeletalMesh|SetMorphTarget (Variables|Default|Getwoman) "happy" _newtrack_0_3 true))))))))

(event Game|Damage|EventAnyDamage
  (params (Damage :type Float%20%28single-precision%29) (DamageType :type Damage%20Type%20Object%20Reference) (InstigatedBy :type Controller%20Object%20Reference) (DamageCauser :type Actor%20Object%20Reference))
  (Variables|Default|SetDead true)
  (Collision|SetCollisionEnabled (Variables|Collision|GetCapsuleComponent) "NoCollision")
  (CallFunction|StopFaceAnim))

(fn ConstructionScript)