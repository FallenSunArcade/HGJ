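; Robert character Blueprint: an NPC with morph-target facial animation on the Man mesh and random wandering.
; Tick plays three nested timelines driving eye and happy morphs; StopFaceAnim stops the outer one.
; BeginPlay randomizes Death12 and RandomAnimationStart, which NewShape rerolls.
; Moving sends it to random nearby points unless dead, but its timer is disconnected, as are death handling and body, scale and clothing-color randomization.
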(event Custom|NewShape
  (bind _output_get (Variables|Default|SetRandomAnimationStart (Math|Random|RandomFloatinRange 0.0 1.0)))
  (Development|PrintString (Utilities|String|ToString(Float) _output_get)))

(event Custom|StopFaceAnim
  (bind _newtrack_0 (Timeline|Timeline Stop)
    (:Update
      (Components|SkeletalMesh|SetMorphTarget (Variables|Default|GetMan) "eyesclosed" _newtrack_0 true)
      (bind _newtrack_0_2 (Timeline|Timeline_0 Play)
        (:Update
          (Components|SkeletalMesh|SetMorphTarget (Variables|Default|GetMan) "eyessmall" _newtrack_0_2 true)
          (bind _newtrack_0_3 (Timeline|Timeline_1 Play)
            (:Update
              (Components|SkeletalMesh|SetMorphTarget (Variables|Default|GetMan) "happy" _newtrack_0_3 true))))))))

(event Custom|Moving
  (bind _asbp_player (Utilities|Casting|CastToBP_Player (Game|GetPlayerCharacter 0)))
  (if (not (Variables|Default|GetDead))
    (AI|AIMoveTo self (.RandomLocation (AI|Navigation|GetRandomReachablePointinRadius (Transformation|GetActorLocation) 1e+03 0 0)) 0 1e+02 true)))

(event EventBeginPlay
  (Variables|Default|SetDeath12 (Math|Random|RandomBool))
  (bind _output_get (Variables|Default|SetRandomAnimationStart (Math|Random|RandomFloatinRange 0.0 1.0)))
  (Development|PrintString (Utilities|String|ToString(Float) _output_get)))

(event Collision|EventActorBeginOverlap
  (params (OtherActor :type Actor%20Object%20Reference)))

(event EventTick
  (params (DeltaSeconds :type Float%20%28single-precision%29))
  (bind _newtrack_0 (Timeline|Timeline Play)
    (:Update
      (Components|SkeletalMesh|SetMorphTarget (Variables|Default|GetMan) "eyesclosed" _newtrack_0 true)
      (bind _newtrack_0_2 (Timeline|Timeline_0 Play)
        (:Update
          (Components|SkeletalMesh|SetMorphTarget (Variables|Default|GetMan) "eyessmall" _newtrack_0_2 true)
          (bind _newtrack_0_3 (Timeline|Timeline_1 Play)
            (:Update
              (Components|SkeletalMesh|SetMorphTarget (Variables|Default|GetMan) "happy" _newtrack_0_3 true))))))))

(event Game|Damage|EventAnyDamage
  (params (Damage :type Float%20%28single-precision%29) (DamageType :type Damage%20Type%20Object%20Reference) (InstigatedBy :type Controller%20Object%20Reference) (DamageCauser :type Actor%20Object%20Reference)))

(fn ConstructionScript)