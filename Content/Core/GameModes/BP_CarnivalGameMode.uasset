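; Carnival game mode that plays FMOD dialog voice lines and handles the return to the main menu.
; Speaking reads the current dialog section from the game instance and passes the matching event to SectionVoiceActing.
; That stops the previous instance, plays the new one, then sets the section-named parameter to the line index.
; ExitToMenu waits briefly, resets game state and dialog section, then opens the menu map.
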(event Custom|Exit%20To%20Menu
  (Utilities|FlowControl|Delay 3.0)
  (bind _asbp_game_instance (Utilities|Casting|CastToBP_GameInstance (Game|GetGameInstance)))
  (Class|HGGameInstance|SetGameState _asbp_game_instance "ShootingBooth")
  (Class|HGGameInstance|SetCurrentDialogSection _asbp_game_instance "Section1")
  (Game|OpenLevel(byObjectReference) "/Game/Maps/Menu/MenuMap.MenuMap"))

(event EventSpeaking
  (params (Index :type Float%20%28single-precision%29))
  (Variables|Default|SetCurrentIndex Index)
  (bind _asbp_game_instance (Utilities|Casting|CastToBP_GameInstance (Game|GetGameInstance)))
  (switch Utilities|FlowControl|Switch|SwitchonEDialogSections (Class|HGGameInstance|GetCurrentDialogSection _asbp_game_instance)
    (:Section1
      (Utilities|SectionVoiceActing "/Game/FMOD/Events/Dialog/Section1.Section1" "Section1"))
    (:Section2
      (Utilities|SectionVoiceActing "/Game/FMOD/Events/Dialog/Section2.Section2" "Section2"))
    (:Section3
      (Utilities|SectionVoiceActing "/Game/FMOD/Events/Dialog/Section3.Section3" "Section3"))
    (:Section4
      (Utilities|SectionVoiceActing "/Game/FMOD/Events/Dialog/Section4.Section4" "Section4"))
    (:Section5
      (Utilities|SectionVoiceActing "/Game/FMOD/Events/Dialog/Section5.Section5" "Section5"))
    (:Section6
      (Utilities|SectionVoiceActing "/Game/FMOD/Events/Dialog/Section6.Section6" "Section6"))
    (:Section7
      (Utilities|SectionVoiceActing "/Game/FMOD/Events/Dialog/Section7.Section7" "Section7"))
    (:Section8
      (Utilities|SectionVoiceActing "/Game/FMOD/Events/Dialog/Section8.Section8" "Section8"))
    (:Section9
      (Utilities|SectionVoiceActing "/Game/FMOD/Events/Dialog/Section9.Section9" "Section9"))))

(fn ConstructionScript)