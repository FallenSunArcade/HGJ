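; Actor component that runs dialog interactions, using a Behavior Tree as the dialog graph.
; It spawns its own AIController at BeginPlay; on interaction it shows WBP_Dialog and runs DialogTree, passing the widget and owner through the BB_Dialog blackboard.
; Widget events switch input mode: pause and resume toggle visibility, while exit stops the tree and removes the widget.
; SetDialogTree swaps the tree used for later interactions.
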(event Custom|OnExit_Event
  (bind _dialogwidget (Variables|Default|GetDialogWidget))
  (bind _returnvalue (Widget|GetOwningPlayer _dialogwidget))
  (Input|SetInputModeGameOnly _returnvalue false)
  (Variables|/Script/Engine.PlayerController|SetbShowMouseCursor _returnvalue false)
  (AI|Logic|StopLogic (Variables|/Script/AIModule.AIController|GetBrainComponent (Variables|Default|GetAIController)) "Dialog Exited")
  (Widget|RemovefromParent (Variables|Default|GetDialogWidget)))

(event Custom|OnResumeEvent
  (bind _dialogwidget (Variables|Default|GetDialogWidget))
  (Input|SetInputModeUIOnly (Widget|GetOwningPlayer _dialogwidget) _dialogwidget "DoNotLock" false)
  (Variables|/Script/UMG.Widget|SetVisibility _dialogwidget "Visible"))

(event Custom|OnPause_Event
  (bind _dialogwidget (Variables|Default|GetDialogWidget))
  (bind _returnvalue (Widget|GetOwningPlayer _dialogwidget))
  (Input|SetInputModeGameOnly _returnvalue false)
  (Variables|/Script/Engine.PlayerController|SetbShowMouseCursor _returnvalue false)
  (Variables|/Script/UMG.Widget|SetVisibility _dialogwidget "Hidden"))

(event EventBeginPlay
  (bind _returnvalue (Game|SpawnActorfromClass "/Script/AIModule.AIController" (Math|Transform|MakeTransform "0, 0, 0" "0, 0, 0" "1.000000,1.000000,1.000000") "Undefined" 0 0))
  (Variables|Default|SetAIController _returnvalue))

(event EventOnInteraction
  (params (PlayerCharacter :type BP%20Player%20Object%20Reference))
  (bind _returnvalue (Pawn|GetController PlayerCharacter))
  (bind _asplayer_controller (Utilities|Casting|CastToPlayerController _returnvalue))
  (Variables|Default|SetPlayer PlayerCharacter)
  (bind _returnvalue_2 (UserInterface|CreateWidget "/Game/Core/DialogSystem/WBP_Dialog.WBP_Dialog_C" _asplayer_controller))
  (bind _output_get (Variables|Default|SetDialogWidget _returnvalue_2))
  (EventDispatchers|AssignOnExit _output_get (delegate Custom|OnExit_Event))
  (EventDispatchers|BindEventtoOnPause _output_get (delegate Custom|OnPause_Event))
  (EventDispatchers|BindEventtoOnResume _output_get (delegate Custom|OnResumeEvent))
  (UserInterface|Viewport|AddtoViewport _output_get 0)
  (Input|SetInputModeUIOnly _asplayer_controller _output_get "DoNotLock" true)
  (Variables|/Script/Engine.PlayerController|SetbShowMouseCursor _asplayer_controller true)
  (AI|RunBehaviorTree (Variables|Default|GetAIController) (Variables|Default|GetDialogTree))
  (bind _blackboardcomponent (Class|AIController|UseBlackboard (Variables|Default|GetAIController) "/Game/Core/DialogSystem/BB_Dialog.BB_Dialog"))
  (AI|Components|Blackboard|SetValueasObject _blackboardcomponent (Utilities|Name|MakeLiteralName "DialogWidget") (Variables|Default|GetDialogWidget))
  (AI|Components|Blackboard|SetValueasObject _blackboardcomponent (Utilities|Name|MakeLiteralName "Owner") (Components|GetOwner)))

(fn SetDialogTree
  (params (DialogTree :type Behavior%20Tree%20Object%20Reference))
  (Variables|Default|SetDialogTree DialogTree))