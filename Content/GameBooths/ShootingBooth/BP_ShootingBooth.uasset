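; BP_ShootingBooth is the carnival shooting game booth actor, handling the booth's audio and exposing its shooting position.
; BeginPlay starts carnival music through FMOD at the booth's location and sets its Dark_Layer parameter to zero if the instance is valid.
; RoundStart and RoundOver play start, win or game-over sounds at the same location, with the Won flag choosing the ending.
; GetShootingPosition returns the stored shooting position.
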(event EventBeginPlay
  (bind _returnvalue (Class|FMODBlueprintStatics|PlayEventatLocation "/Game/FMOD/Events/Music/Music_carnival.Music_carnival" (Math|Conversions|ToTransform(Vector) (Transformation|GetActorLocation))))
  (Class|FMODBlueprintStatics|EventInstancePlay _returnvalue)
  (bind _returnvalue_2 (Class|FMODBlueprintStatics|EventInstanceIsValid _returnvalue))
  (if _returnvalue_2
    (Class|FMODBlueprintStatics|EventInstanceSetParameter _returnvalue "Dark_Layer" 0.0)))

(event EventRoundStart
  (params (RoundNumber :type Integer))
  (Class|FMODBlueprintStatics|PlayEventatLocation "/Game/FMOD/Events/Booths/Game_Start.Game_Start" (Math|Conversions|ToTransform(Vector) (Transformation|GetActorLocation))))

(event EventRoundOver
  (params (Won :type Boolean))
  (bind _returnvalue (Transformation|GetActorLocation))
  (bind _returnvalue_2 (Math|Conversions|ToTransform(Vector) _returnvalue))
  (if Won
    (Class|FMODBlueprintStatics|PlayEventatLocation "/Game/FMOD/Events/Booths/Game_Won.Game_Won" _returnvalue_2)
    (else
      (Class|FMODBlueprintStatics|PlayEventatLocation "/Game/FMOD/Events/Booths/Game_Over.Game_Over" _returnvalue_2))))

(fn ConstructionScript)

(fn GetShootingPosition
  (return (Variables|Default|GetShootingPostion)))