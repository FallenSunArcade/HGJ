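; Whack-a-mole carnival booth that switches its mole targets on and off with each round and exposes a playing position.
; RoundStart and RoundOver use WhackAMoleGame to set GameHasStarted on seven BP_TargetMole child actors.
; FMOD events play at the booth for round start, win and loss.
; BeginPlay also starts the carnival music there, with its Dark_Layer parameter zeroed.
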(event EventBeginPlay
  (bind _returnvalue (Class|FMODBlueprintStatics|PlayEventatLocation "/Game/FMOD/Events/Music/Music_carnival.Music_carnival" (Math|Conversions|ToTransform(Vector) (Transformation|GetActorLocation))))
  (Class|FMODBlueprintStatics|EventInstancePlay _returnvalue)
  (bind _returnvalue_2 (Class|FMODBlueprintStatics|EventInstanceIsValid _returnvalue))
  (if _returnvalue_2
    (Class|FMODBlueprintStatics|EventInstanceSetParameter _returnvalue "Dark_Layer" 0.0)))

(event EventRoundStart
  (params (RoundNumber :type Integer))
  (Utilities|FlowControl|Sequence
    (:then_0
      (Utilities|WhackAMoleGame (Variables|Default|GetTargetMole) true))
    (:then_1
      (Utilities|WhackAMoleGame (Variables|Default|GetTargetMole1) true))
    (:then_2
      (Utilities|WhackAMoleGame (Variables|Default|GetTargetMole2) true))
    (:then_3
      (Utilities|WhackAMoleGame (Variables|Default|GetTargetMole3) true))
    (:then_4
      (Utilities|WhackAMoleGame (Variables|Default|GetTargetMole4) true))
    (:then_5
      (Utilities|WhackAMoleGame (Variables|Default|GetTargetMole5) true))
    (:then_6
      (Utilities|WhackAMoleGame (Variables|Default|GetTargetMole6) true))
    (:then_7
      (Class|FMODBlueprintStatics|PlayEventatLocation "/Game/FMOD/Events/Booths/Game_Start.Game_Start" (Math|Conversions|ToTransform(Vector) (Transformation|GetActorLocation))))))

(event EventRoundOver
  (params (Won :type Boolean))
  (bind _returnvalue (Transformation|GetActorLocation))
  (bind _returnvalue_2 (Math|Conversions|ToTransform(Vector) _returnvalue))
  (Utilities|FlowControl|Sequence
    (:then_0
      (Utilities|WhackAMoleGame (Variables|Default|GetTargetMole) false))
    (:then_1
      (Utilities|WhackAMoleGame (Variables|Default|GetTargetMole1) false))
    (:then_2
      (Utilities|WhackAMoleGame (Variables|Default|GetTargetMole2) false))
    (:then_3
      (Utilities|WhackAMoleGame (Variables|Default|GetTargetMole3) false))
    (:then_4
      (Utilities|WhackAMoleGame (Variables|Default|GetTargetMole4) false))
    (:then_5
      (Utilities|WhackAMoleGame (Variables|Default|GetTargetMole5) false))
    (:then_6
      (Utilities|WhackAMoleGame (Variables|Default|GetTargetMole6) false))
    (:then_7
      (if Won
        (Class|FMODBlueprintStatics|PlayEventatLocation "/Game/FMOD/Events/Booths/Game_Won.Game_Won" _returnvalue_2)
        (else
          (Class|FMODBlueprintStatics|PlayEventatLocation "/Game/FMOD/Events/Booths/Game_Over.Game_Over" _returnvalue_2))))))

(fn ConstructionScript)

(fn GetPlayingPosition
  (return (Variables|Default|GetPlayingPosition)))