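; Wheel of Misfortune booth that spins its wheel and sends the player into the first Dreamworld level.
; SpinTheWheel plays a timeline that scales the RotatingMovement rotation rate and, on its first update, adds an FMOD audio component through a DoOnce.
; A five-second timer started alongside the spin calls LoadDreamWorld, which opens Lvl2_Dreamworld1 and sets the game instance's state to DreamWorld1.
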(event Custom|SpinTheWheel
  ;[1 1 1] Rotation
  (Variables|Default|SetTarget 2e+01)
  (Utilities|Time|SetTimerbyFunctionName 0 "LoadDreamWorld" 5.0)
  (bind _newtrack_0 (Timeline|Timeline_0 Play)
    (:Update
      (Variables|/Script/Engine.RotatingMovementComponent|SetRotationRate (Variables|Default|GetRotatingMovement) (Math|Rotator|MakeRotator 0.0 (* _newtrack_0 (Variables|Default|GetTarget)) 0.0))
      (Utilities|FlowControl|DoOnce false
        (:Completed
          (AddComponent|AddFMODAudioComponent false))))))

(fn ConstructionScript)

(fn LoadDreamWorld
  (Game|OpenLevel(byObjectReference) "/Game/Maps/Lvl2_Dreamworld1.Lvl2_Dreamworld1")
  (bind _asbp_game_instance (Utilities|Casting|CastToBP_GameInstance (Game|GetGameInstance)))
  (Class|HGGameInstance|SetGameState _asbp_game_instance "DreamWorld1"))