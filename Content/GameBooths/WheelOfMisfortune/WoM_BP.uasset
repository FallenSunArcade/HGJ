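; Wheel of Misfortune game booth Blueprint that spins a wheel, currently triggered by a debug overlap.
; The first overlap of InteractionRange by an actor whose first tag is "Player" prints a debug message and calls SpinTheWheel once.
; A timeline curve scaled by Target drives the RotatingMovement yaw rate, and its first update adds an FMOD audio component.
; The example node that sets Target is unconnected.
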(event OnComponentBeginOverlap(InteractionRange)
  (params (OverlappedComponent :type Primitive%20Component%20Object%20Reference) (OtherActor :type Actor%20Object%20Reference) (OtherComp :type Primitive%20Component%20Object%20Reference) (OtherBodyIndex :type Integer) (bFromSweep :type Boolean) (SweepResult :type Hit%20Result%20Structure%20%28by%20ref%29))
  (bind _tags (Variables|/Script/Engine.Actor|GetTags OtherActor))
  ;[1 1 1] Debug Activation
  (if (Utilities|Array|IsValidIndex _tags)
    (if (== (Utilities|Array|Get(acopy) _tags) "Player")
      (Utilities|FlowControl|DoOnce false
        (:Completed
          (Development|PrintString "Hello")
          (CallFunction|SpintheWheel))))))

(event Custom|SpinTheWheel
  ;[1 1 1] Rotation
  (bind _newtrack_0 (Timeline|Timeline_0 Play)
    (:Update
      (Variables|/Script/Engine.RotatingMovementComponent|SetRotationRate (Variables|Default|GetRotatingMovement) (Math|Rotator|MakeRotator 0.0 (* _newtrack_0 (Variables|Default|GetTarget)) 0.0))
      (Utilities|FlowControl|DoOnce false
        (:Completed
          (AddComponent|AddFMODAudioComponent false))))))

(fn ConstructionScript)